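; BP_PlasmaBolt is a slow-or-fast configurable plasma projectile that damages nearby enemies as it flies, expiring after about eight seconds.
; Tick moves it forward by Speed per frame, unscaled by delta time and without sweep.
; A Delay on Tick throttles damage to I_Enemy actors inside the scaled DamageArea, drawing red debug lines to each.
; Sphere overlap destroys it on anything except enemies and player weapons.
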(event `self.ReceiveBeginPlay`
  (bind _damageareasize (`self.DamageAreaSize`))
  (`KismetSystemLibrary.Delay` 0.1)
  (`SceneComponent.SetRelativeScale3D` (`self.DamageArea`) (`KismetMathLibrary.MakeVector` _damageareasize _damageareasize _damageareasize))
  (`KismetSystemLibrary.Delay` 8.0)
  (`self.K2_DestroyActor`))

(event `self.ReceiveTick`
  (params (DeltaSeconds :type "Float (single-precision)"))
  (`|ExecutionSequence`
    (:`then_0`
      (`KismetSystemLibrary.Delay` 0.1)
      (for _array_element (`PrimitiveComponent.GetOverlappingActors` (`self.DamageArea`) null)
        (if (`KismetSystemLibrary.DoesImplementInterface` _array_element "/Game/VRLocomotionTemplate/ZOldAssets/Blueprints/Interface/I_Enemy.I_Enemy_C")
          (`GameplayStatics.ApplyDamage` _array_element (`self.Damage`) null null "/Script/Engine.DamageType")
          (`KismetSystemLibrary.DrawDebugLine` (`SceneComponent.K2_GetComponentLocation` (`self.Bullet`)) (`self.K2_GetActorLocation` _array_element) (struct :`R` 1.0 :`A` 1.0) 0.05 5.0))))
    (:`then_1`
      ;[1 1 1] MoveActor Forward
      (`self.K2_SetActorLocation` (+ (`self.K2_GetActorLocation`) (* (`KismetMathLibrary.GetForwardVector` (`self.K2_GetActorRotation`)) (`self.Speed`)))))))

(event `self.Sphere.OnComponentBeginOverlap`
  (params (OverlappedComponent :type "PrimitiveComponent Object Reference") (OtherActor :type "Actor Object Reference") (OtherComp :type "PrimitiveComponent Object Reference") (OtherBodyIndex :type Integer) (bFromSweep :type Boolean) (SweepResult :type "HitResult Structure (by ref)"))
  (if (!= OtherActor self)
    (if (`KismetSystemLibrary.DoesImplementInterface` OtherActor "/Game/VRLocomotionTemplate/ZOldAssets/Blueprints/Interface/I_Enemy.I_Enemy_C")
      _
      (elif (not (`KismetSystemLibrary.DoesImplementInterface` OtherActor "/Game/VRLocomotionTemplate/ZOldAssets/Blueprints/Interface/I_PlayerWeapon.I_PlayerWeapon_C"))
        (`self.K2_DestroyActor`)))))

(fn `UserConstructionScript`)