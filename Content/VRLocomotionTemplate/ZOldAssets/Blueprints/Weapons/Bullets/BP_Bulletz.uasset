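; BP_Bulletz is a physics-driven projectile that damages enemies and the player and can be deflected by shields.
; Capsule overlaps damage I_Enemy actors or a matching player component (commented as the head), while BP_Sheild hits reflect the mesh's velocity via FindMirrorVector.
; StartPhysics and StopPhysics launch and halt the mesh.
; Niagara trail-length and timed-destroy logic is disconnected, and Begin Play and Tick are empty.
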(event `self.ReceiveBeginPlay`
  ;[1 1 1] Begin Play
)

(event `self.ReceiveTick`
  (params (DeltaSeconds :type "Float (single-precision)"))
  ;[1 1 1] Event Tick
)

(event `self.Capsule.OnComponentBeginOverlap`
  (params (OverlappedComponent :type "PrimitiveComponent Object Reference") (OtherActor :type "Actor Object Reference") (OtherComp :type "PrimitiveComponent Object Reference") (OtherBodyIndex :type Integer) (bFromSweep :type Boolean) (SweepResult :type "HitResult Structure (by ref)"))
  (bind _staticmesh (`self.StaticMesh`))
  ;[1 1 1] Collisions
  (if (`KismetSystemLibrary.DoesImplementInterface` OtherActor "/Game/VRLocomotionTemplate/ZOldAssets/Blueprints/Interface/I_Enemy.I_Enemy_C")
    ;;[0.005281 1 0] Hits Enemy
    (`GameplayStatics.ApplyDamage` OtherActor (`self.Damage`) null null "/Script/Engine.DamageType")
    (elif (`KismetSystemLibrary.DoesImplementInterface` OtherActor "/Game/VRLocomotionTemplate/ZOldAssets/Blueprints/Interface/I_PlayerWeapon.I_PlayerWeapon_C")
      ;;[1 0.5811 0] Hits Shield
      (bind _asbp_sheild (cast `/Game/VRLocomotionTemplate/ZOldAssets/Blueprints/Weapons/BP_Sheild` OtherActor))
      (`/Engine/EditorBlueprintResources/StandardMacros.IsValid` _asbp_sheild
        (:`Is Valid`
          (bind _sheild (`/Game/VRLocomotionTemplate/ZOldAssets/Blueprints/Weapons/BP_Sheild.Sheild` _asbp_sheild))
          (bind _mirroredvector (`self.FindMirrorVector` (`KismetMathLibrary.GetForwardVector` (`self.K2_GetActorRotation`)) (`SceneComponent.GetForwardVector` _sheild)))
          (bind _returnvalue (`SceneComponent.K2_GetComponentLocation` _sheild))
          (bind _returnvalue_2 (* _mirroredvector (`self.Speed`)))
          (bind (_returnvalue_roll _returnvalue_pitch _returnvalue_yaw) (`KismetMathLibrary.BreakRotator` (`KismetMathLibrary.FindLookAtRotation` _returnvalue (+ _returnvalue _returnvalue_2))))
          (`SceneComponent.K2_SetWorldRotation` _staticmesh (`KismetMathLibrary.MakeRotator` _returnvalue_pitch _returnvalue_roll (+ _returnvalue_yaw 90.0)) false false)
          (`PrimitiveComponent.SetPhysicsLinearVelocity` _staticmesh (0.0 0.0 0.0) false "None")
          (`PrimitiveComponent.AddImpulse` _staticmesh _returnvalue_2 "None" true)
          (set `self.distanceTravel` 0.0)))
      (else
        ;;[1 0 0] Collision With Player Head
        (if (== OtherComp null)
          (`GameplayStatics.ApplyDamage` OtherActor (`self.Damage`)))))))

(event `StopPhysics`
  (`PrimitiveComponent.SetPhysicsLinearVelocity` (`self.StaticMesh`) (0.0 0.0 0.0) false "None")
  (set `self.Moving` false))

(event `StartPhysics`
  (bind _staticmesh (`self.StaticMesh`))
  (`PrimitiveComponent.AddImpulse` _staticmesh (* (`SceneComponent.GetForwardVector` _staticmesh) (`self.Speed`)) "None" true)
  (set `self.Moving` true))

(fn `FindMirrorVector`
  (params (InputVector :type "Vector Structure") (Normal :type "Vector Structure"))
  (returns (MirroredVector :type "Vector Structure"))
  (return (- InputVector (* (* Normal (`KismetMathLibrary.Dot_VectorVector` InputVector Normal)) 2.0))))

(fn `UserConstructionScript`)