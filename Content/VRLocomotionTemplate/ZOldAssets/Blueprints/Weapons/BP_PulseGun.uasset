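; BP_PulseGun is a charge-up gun that fires a BP_PlasmaBolt when released with enough charge.
; IsShooting sets the firing flag and controls a looping rising sound.
; While held, Tick uses a Delay to step up charge, shifting two lights from red to green and growing a sphere.
; On release, Shoot spawns a bolt with charge-scaled size and damage, plays a sound and resets charge and visuals; insufficient charge is discarded.
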(event `self.ReceiveBeginPlay`
  (`LightComponent.SetLightColor` (`self.PointLight`) (make `LinearColor` 1.0) true)
  (`LightComponent.SetLightColor` (`self.PointLight1`) (make `LinearColor` 1.0) true))

(event `self.ReceiveTick`
  (params (DeltaSeconds :type "Float (single-precision)"))
  (bind _returnvalue (/ (`self.CurrentChargeAmount`) (`self.FullChrage`)))
  (bind _returnvalue_2 (+ (* (/ (`self.CurrentChargeAmount`) (`self.FullChrage`)) 10.0) 0.5))
  (if (`self.Shooting`)
    (`KismetSystemLibrary.Delay` 0.05)
    (set `self.CurrentChargeAmount` (`KismetMathLibrary.FClamp` (+ (`self.CurrentChargeAmount`) 0.05) 0.0 (`self.FullChrage`)))
    (`LightComponent.SetLightColor` (`self.PointLight`) (make `LinearColor` (- 1.0 _returnvalue) _returnvalue) true)
    (`LightComponent.SetLightColor` (`self.PointLight1`) (make `LinearColor` (- 1.0 _returnvalue) _returnvalue) true)
    (`SceneComponent.SetRelativeScale3D` (`self.Sphere`) (`KismetMathLibrary.MakeVector` _returnvalue_2 _returnvalue_2 _returnvalue_2))
    (elif (>= (`self.CurrentChargeAmount`) (`self.MinCharge`))
      (`self.Shoot`)
      (else
        (set `self.CurrentChargeAmount` 0.0)))))

(fn `ChrageUp`)

(fn `IsShooting`
  (params (bShooting :type Boolean))
  (bind _chrageupsound (`self.ChrageUpSound`))
  (bind _output_get (set `self.Shooting` bShooting))
  (if _output_get
    (bind _returnvalue (`GameplayStatics.SpawnSoundAttached` "/Game/VRLocomotionTemplate/Audio/SoundFiles/Weapon/Endless_Rising_-_Loop.Endless_Rising_-_Loop" (`self.StaticMesh`) "None" (0.0 0.0 0.0) (struct) "KeepRelativeOffset" false 1.0 1.0 0.0 null null))
    (set `self.ChrageUpSound` _returnvalue)
    (else
      (`/Engine/EditorBlueprintResources/StandardMacros.IsValid` _chrageupsound
        (:`Is Valid`
          (`AudioComponent.Stop` _chrageupsound)
          (`ActorComponent.K2_DestroyComponent` _chrageupsound))))))

(fn `Shoot`
  (bind (_returnvalue_location _returnvalue_rotation) (`KismetMathLibrary.BreakTransform` (`SceneComponent.K2_GetComponentToWorld` (`self.Scene`))))
  (bind _returnvalue (+ (* (/ (`self.CurrentChargeAmount`) (`self.FullChrage`)) 10.0) 0.5))
  (bind _returnvalue_2 (`|SpawnActorFromClass` "/Game/VRLocomotionTemplate/ZOldAssets/Blueprints/Weapons/Bullets/BP_PlasmaBolt.BP_PlasmaBolt_C" (`KismetMathLibrary.MakeTransform` _returnvalue_location _returnvalue_rotation (`KismetMathLibrary.MakeVector` _returnvalue _returnvalue _returnvalue)) "Undefined" "OverrideRootScale" null null))
  (`/Engine/EditorBlueprintResources/StandardMacros.IsValid` _returnvalue_2
    (:`Is Valid`
      (set `/Game/VRLocomotionTemplate/ZOldAssets/Blueprints/Weapons/Bullets/BP_PlasmaBolt.Speed` (`self.ProjectileSpeed`) _returnvalue_2)
      (set `/Game/VRLocomotionTemplate/ZOldAssets/Blueprints/Weapons/Bullets/BP_PlasmaBolt.Damage` (* (`self.CurrentChargeAmount`) (`self.DamageMultiplier`) (`self.BaseDamage`)) _returnvalue_2)
      (set `/Game/VRLocomotionTemplate/ZOldAssets/Blueprints/Weapons/Bullets/BP_PlasmaBolt.DamageAreaSize` (`self.DamageArea`) _returnvalue_2))
    (:`Is Not Valid`
      _))
  (`GameplayStatics.PlaySoundAtLocation` "/Game/VRLocomotionTemplate/Audio/SoundFiles/Weapon/29_Minigun_Fire_M_V1_RO.29_Minigun_Fire_M_V1_RO" (`self.K2_GetActorLocation`) (struct) 1.0 1.0 0.0 null null null)
  (set `self.CurrentChargeAmount` 0.0)
  (`LightComponent.SetLightColor` (`self.PointLight`) (make `LinearColor` 1.0) true)
  (`LightComponent.SetLightColor` (`self.PointLight1`) (make `LinearColor` 1.0) true)
  (`SceneComponent.SetRelativeScale3D` (`self.Sphere`) (0.01 0.01 0.01)))

(fn `UserConstructionScript`)