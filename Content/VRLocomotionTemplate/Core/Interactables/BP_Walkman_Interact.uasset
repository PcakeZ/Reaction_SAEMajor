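; Walkman interactable for the VR locomotion template that can be highlighted, picked up by hand and launched by a distance grab.
; Hover and grab-hover outline the mesh through custom depth with different stencil values, and ending hover also detaches the actor.
; Interaction disables physics and attaches to the hand, then release detaches and restores physics.
; Grabbing applies a velocity-change impulse, with a timed Moving flag blocking repeat launches.
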(event `/Game/VRLocomotionTemplate/Core/Interactables/I_Interactable.StartHover`
  (bind _staticmesh (`self.StaticMesh`))
  ;[1 1 1] Highlight Object
  (`PrimitiveComponent.SetRenderCustomDepth` _staticmesh true)
  (`PrimitiveComponent.SetCustomDepthStencilValue` _staticmesh 2))

(event `/Game/VRLocomotionTemplate/Core/Interactables/I_Interactable.EndHover`
  ;[1 1 1] Highlight Object
  (`PrimitiveComponent.SetRenderCustomDepth` (`self.StaticMesh`) false)
  (`self.K2_DetachFromActor` "KeepWorld" "KeepWorld" "KeepWorld"))

(event `/Game/VRLocomotionTemplate/Core/Interactables/I_Interactable.StartInteract`
  (params (Hand :type "SceneComponent Object Reference") (GunPos :type "SceneComponent Object Reference"))
  ;[1 1 1] Pickup Object
  (`PrimitiveComponent.SetSimulatePhysics` (`self.StaticMesh`) false)
  (`self.K2_AttachToComponent` Hand "None" "KeepWorld" "KeepWorld" "KeepWorld"))

(event `/Game/VRLocomotionTemplate/Core/Interactables/I_Interactable.EndInteract`
  ;[1 1 1] Pickup Object
  (`PrimitiveComponent.SetSimulatePhysics` (`self.StaticMesh`) true)
  (`self.K2_DetachFromActor` "KeepWorld" "KeepWorld" "KeepWorld"))

(event `StartGrab`
  (params (LaunchVelocity :type "Vector Structure") (Time :type "Float (double-precision)"))
  (if (not (`self.Moving`))
    (`PrimitiveComponent.AddImpulse` (`self.StaticMesh`) LaunchVelocity "None" true)
    (set `self.Moving` true)
    (`KismetSystemLibrary.Delay` Time)
    (set `self.Moving` false)))

(event `StartGrabHover`
  (bind _staticmesh (`self.StaticMesh`))
  (`PrimitiveComponent.SetRenderCustomDepth` _staticmesh true)
  (`PrimitiveComponent.SetCustomDepthStencilValue` _staticmesh 3))

(event `EndGrabHover`
  (`PrimitiveComponent.SetRenderCustomDepth` (`self.StaticMesh`) false))

(fn `UserConstructionScript`)