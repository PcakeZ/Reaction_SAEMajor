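; BP_Keypad is an interactable VR environment keypad that triggers a linked object when something overlaps its box.
; While not Active, it accepts either a specific Key actor when NeedsKey is set, or the player pawn otherwise.
; A valid overlap sends Trigger1 to ObjectToTrigger, swaps the visible cube mesh and plays a button-press sound.
; The graph never sets Active, so valid overlaps can fire it repeatedly unless that flag changes elsewhere.
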(event `self.Box.OnComponentBeginOverlap`
  (params (OverlappedComponent :type "PrimitiveComponent Object Reference") (OtherActor :type "Actor Object Reference") (OtherComp :type "PrimitiveComponent Object Reference") (OtherBodyIndex :type Integer) (bFromSweep :type Boolean) (SweepResult :type "HitResult Structure (by ref)"))
  (if (`self.active`)
    _
    (elif (`self.NeedsKey`)
      (if (== OtherActor (`self.Key`))
        (message `/Game/VRLocomotionTemplate/Core/Interactables/Environment/I_Activate.Trigger_1` (`self.ObjectToTrigger`) :!label _label)
        (`SceneComponent.SetVisibility` (`self.Cube1`) true false)
        (`SceneComponent.SetVisibility` (`self.Cube`) false false)
        (`GameplayStatics.PlaySoundAtLocation` "/Game/VRLocomotionTemplate/Audio/SoundFiles/QA1/Applied/35_R_ButtonPress_M_V2_RO.35_R_ButtonPress_M_V2_RO" (`SceneComponent.K2_GetComponentLocation` (`self.Cube`)) (struct) 0.4 (`GameplayStatics.GetWorldDeltaSeconds`) 0.0 "/Game/VRLocomotionTemplate/Audio/Attenuations/AT_Footstep.AT_Footstep" null null))
      (else
        (cast `/Game/VRLocomotionTemplate/Core/Characters/BP_PlayerPawn` OtherActor)
        (goto _label)))))

(fn `UserConstructionScript`)