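; BP_DuelButtonPress is one of a linked pair of VR environment buttons that fire a target only when both have been triggered.
; Box overlap events compare the overlapped component, not the other component, to the player pawn's two cubes before setting Triggered.
; When triggered, it checks its linked OtherButton and sends Trigger1Message to the target if both are set.
; End overlap clears Triggered only when already false, so a press latches.
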(event `self.ReceiveBeginPlay`
  (bind _asbp_player_pawn (cast `/Game/VRLocomotionTemplate/Core/Characters/BP_PlayerPawn` (`GameplayStatics.GetPlayerPawn` 0)))
  (set `self.Player` _asbp_player_pawn))

(event `self.Box.OnComponentBeginOverlap`
  (params (OverlappedComponent :type "PrimitiveComponent Object Reference") (OtherActor :type "Actor Object Reference") (OtherComp :type "PrimitiveComponent Object Reference") (OtherBodyIndex :type Integer) (bFromSweep :type Boolean) (SweepResult :type "HitResult Structure (by ref)"))
  (bind _player (`self.Player`))
  (if (and (not (`self.Triggered`)) (or (== OverlappedComponent (`/Game/VRLocomotionTemplate/Core/Characters/BP_PlayerPawn.Cube` _player)) (== OverlappedComponent (`/Game/VRLocomotionTemplate/Core/Characters/BP_PlayerPawn.Cube1` _player))))
    (set `self.Triggered` true)
    (bind _asbp_duel_button_press (cast `/Game/VRLocomotionTemplate/Core/Interactables/Environment/BP_DuelButtonPress` (`self.OtherButton`)))
    (if (`/Game/VRLocomotionTemplate/Core/Interactables/Environment/BP_DuelButtonPress.Triggered` _asbp_duel_button_press)
      (message `/Game/VRLocomotionTemplate/Core/Interactables/Environment/I_Activate.Trigger_1` (`self.TagetObject`)))))

(event `self.Box.OnComponentEndOverlap`
  (params (OverlappedComponent :type "PrimitiveComponent Object Reference") (OtherActor :type "Actor Object Reference") (OtherComp :type "PrimitiveComponent Object Reference") (OtherBodyIndex :type Integer))
  (bind _player (`self.Player`))
  (if (and (not (`self.Triggered`)) (or (== OverlappedComponent (`/Game/VRLocomotionTemplate/Core/Characters/BP_PlayerPawn.Cube` _player)) (== OverlappedComponent (`/Game/VRLocomotionTemplate/Core/Characters/BP_PlayerPawn.Cube1` _player))))
    (set `self.Triggered` false)))

(fn `UserConstructionScript`)