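; BP_TriggerBox is a one-shot trigger volume in the VR locomotion template, with its box extent set from a variable in the construction script.
; When the cached player pawn first overlaps the box, it sends Trigger1 messages to one object list and a list of valid enemies, and Trigger2 messages to a second object list.
; A Triggered flag then blocks any further activation.
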(event `self.ReceiveBeginPlay`
  (bind _asbp_player_pawn (cast `/Game/VRLocomotionTemplate/Core/Characters/BP_PlayerPawn` (`GameplayStatics.GetPlayerPawn` 0)))
  (set `self.Player` _asbp_player_pawn))

(event `self.Box.OnComponentBeginOverlap`
  (params (OverlappedComponent :type "PrimitiveComponent Object Reference") (OtherActor :type "Actor Object Reference") (OtherComp :type "PrimitiveComponent Object Reference") (OtherBodyIndex :type Integer) (bFromSweep :type Boolean) (SweepResult :type "HitResult Structure (by ref)"))
  (if (`self.Triggered`)
    _
    (elif (== OtherActor (`self.Player`))
      (for _array_element (`self.ObjectstoTrigger`)
        (message `/Game/VRLocomotionTemplate/Core/Interactables/Environment/I_Activate.Trigger_1` _array_element))
      (for _array_element_2 (`self.ObjectstoTrigger2`)
        (message `/Game/VRLocomotionTemplate/Core/Interactables/Environment/I_Activate.Trigger_2` _array_element_2))
      (for _array_element_3 (`self.EnemiesToTrigger`)
        (`/Engine/EditorBlueprintResources/StandardMacros.IsValid` _array_element_3
          (:`Is Valid`
            (message `/Game/VRLocomotionTemplate/Core/Interactables/Environment/I_Activate.Trigger_1` _array_element_3))))
      (set `self.Triggered` true))))

(fn `UserConstructionScript`
  (`BoxComponent.SetBoxExtent` (`self.Box`) (`self.BoxExtent`) true))