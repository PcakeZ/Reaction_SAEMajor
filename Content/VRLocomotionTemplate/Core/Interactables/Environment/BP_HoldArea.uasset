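; BP_HoldArea is a timed trigger zone in the VR locomotion template that starts a countdown when a player pawn or clone enters its box.
; Tick polls the overlap, then latches active, swaps the indicator cubes, plays a sound and sends Trigger1Message to the start target and listed enemies.
; The countdown shows on a text render and messages the target object once at zero.
; Leaving the box does not pause it, as the reset logic is unconnected.
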(event `self.ReceiveBeginPlay`
  (bind _asbp_player_pawn (cast `/Game/VRLocomotionTemplate/Core/Characters/BP_PlayerPawn` (`GameplayStatics.GetPlayerPawn` 0)))
  (set `self.Player` _asbp_player_pawn))

(event `self.ReceiveTick`
  (params (DeltaSeconds :type "Float (single-precision)"))
  (bind _box (`self.Box`))
  (bind _textrender (`self.TextRender`))
  (if (`self.Done`)
    _
    (elif (`self.Activated`)
      (bind _output_get (set `self.TimeLeft` (- (`self.TimeLeft`) DeltaSeconds)))
      (if (<= _output_get 0.0)
        (message `/Game/VRLocomotionTemplate/Core/Interactables/Environment/I_Activate.Trigger_1` (`self.TagetObject`))
        (`TextRenderComponent.K2_SetText` _textrender (`KismetTextLibrary.Conv_DoubleToText` 0.0 "HalfToEven" false true 1 324 2 2))
        (set `self.Done` true)
        (else
          (`TextRenderComponent.K2_SetText` _textrender (`KismetTextLibrary.Conv_DoubleToText` (`self.TimeLeft`) "HalfToEven" false true 1 324 2 2))))
      (elif (> (+ (`KismetArrayLibrary.Array_Length` (`PrimitiveComponent.GetOverlappingActors` _box "/Game/VRLocomotionTemplate/Core/Characters/BP_PlayerPawn.BP_PlayerPawn_C")) (`KismetArrayLibrary.Array_Length` (`PrimitiveComponent.GetOverlappingActors` _box "/Game/VRLocomotionTemplate/Core/Characters/BP_Clone.BP_Clone_C"))) 0)
        (`SceneComponent.SetVisibility` (`self.Cube2`) true false)
        (`SceneComponent.SetVisibility` (`self.Cube`) false false)
        (set `self.Activated` true)
        (message `/Game/VRLocomotionTemplate/Core/Interactables/Environment/I_Activate.Trigger_1` (`self.StartActiveTrigger`))
        (`GameplayStatics.PlaySoundAtLocation` "/Game/VRLocomotionTemplate/Audio/SoundFiles/QA1/Applied/35_R_ButtonPress_M_V2_RO.35_R_ButtonPress_M_V2_RO" (`SceneComponent.K2_GetComponentLocation` (`self.Cube`)) (struct) 0.4 (`GameplayStatics.GetWorldDeltaSeconds`) 0.0 "/Game/VRLocomotionTemplate/Audio/Attenuations/AT_Footstep.AT_Footstep" null null)
        (for _array_element (`self.EnemiesToTrigger`)
          (`/Engine/EditorBlueprintResources/StandardMacros.IsValid` _array_element
            (:`Is Valid`
              (message `/Game/VRLocomotionTemplate/Core/Interactables/Environment/I_Activate.Trigger_1` _array_element))))))))

(fn `UserConstructionScript`)