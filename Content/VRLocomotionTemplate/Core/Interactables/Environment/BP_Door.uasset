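; BP_Door is a VR template environment door: a scalable cube that slides between its starting position and OpenPos.
; Trigger1 opens it and Trigger2 closes it by setting flags that Tick reads.
; Tick eases the cube by a per-frame lerp, stopping within a small tolerance; higher Speed values move it slower because the target is input A.
; The construction script applies the scale and draws a debug box at OpenPos.
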(event `self.ReceiveBeginPlay`
  (set `self.StartPos` (`SceneComponent.K2_GetComponentLocation` (`self.Cube`))))

(event `self.ReceiveTick`
  (params (DeltaSeconds :type "Float (single-precision)"))
  (bind _openpos (`self.OpenPos`))
  (bind _startpos (`self.StartPos`))
  (bind _returnvalue (`SceneComponent.K2_GetComponentLocation` (`self.Cube`)))
  (if (`self.IsMoving`)
    (if (`self.Opening`)
      (`SceneComponent.K2_SetWorldLocation` (`self.Cube`) (`KismetMathLibrary.VLerp` _openpos _returnvalue (`self.Speed`)) false false)
      (if (<= (`KismetMathLibrary.Vector_Distance` _openpos _returnvalue) 5.0)
        (set `self.IsMoving` false))
      (else
        (`SceneComponent.K2_SetWorldLocation` (`self.Cube`) (`KismetMathLibrary.VLerp` _startpos _returnvalue (`self.Speed`)) false false)
        (if (<= (`KismetMathLibrary.Vector_Distance` _startpos _returnvalue) 5.0)
          (set `self.IsMoving` false))))))

(event `/Game/VRLocomotionTemplate/Core/Interactables/Environment/I_Activate.Trigger_1`
  (set `self.IsMoving` true)
  (set `self.Opening` true))

(event `/Game/VRLocomotionTemplate/Core/Interactables/Environment/I_Activate.Trigger_2`
  (set `self.IsMoving` true)
  (set `self.Opening` false))

(fn `UserConstructionScript`
  (bind _cubescale (`self.CubeScale`))
  (`SceneComponent.SetWorldScale3D` (`self.Cube`) _cubescale)
  (`KismetSystemLibrary.DrawDebugBox` (`self.OpenPos`) (* _cubescale 50.0) (struct :`R` 1.0 :`G` 0.279 :`A` 1.0) (`SceneComponent.K2_GetComponentRotation` (`self.Cube`)) 1.0 1.0))