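; BP_WorldPrinter is a world-space text actor that shows a timed sequence of lines accompanied by a demonic voice sound.
; It starts at BeginPlay if Active, or after StartDelay when Trigger1 fires.
; Tick counts down each line's duration, briefly hiding the text and muting the voice between lines.
; After the last line it sends Trigger1Message to linked objects, stops the sound and destroys itself.
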(event `self.ReceiveBeginPlay`
  (bind _asbp_vrgamemode (cast `/Game/VRLocomotionTemplate/Core/GameModes/BP_VRGamemode` (`GameplayStatics.GetGameMode`)))
  (set `self.Gamemode` _asbp_vrgamemode)
  (`TextRenderComponent.K2_SetText` (`self.TextRender`) (`KismetTextLibrary.Conv_StringToText` (`KismetStringLibrary.Concat_StrStr` "")))
  (if (`self.Active`)
    (bind _returnvalue (`GameplayStatics.SpawnSoundAtLocation` "/Game/VRLocomotionTemplate/Audio/DemonicVoice_Cue.DemonicVoice_Cue" (`self.K2_GetActorLocation`) (struct) (`/Game/VRLocomotionTemplate/Core/GameModes/BP_VRGamemode.GameVolume` (`self.Gamemode`)) 1.0 0.0 "/Game/VRLocomotionTemplate/Audio/Attenuations/AT_Footstep.AT_Footstep" null))
    (set `self.SoundRef` _returnvalue)))

(event `self.ReceiveTick`
  (params (DeltaSeconds :type "Float (single-precision)"))
  (bind _soundref (`self.SoundRef`))
  (if (`self.Active`)
    (if (<= (`self.CurrentCooldown`) 0.0)
      (`TextRenderComponent.K2_SetText` (`self.TextRender`) (`|GetArrayItem` (`self.Lines`) (`self.CurrentLine`)))
      (set `self.CurrentCooldown` (`|GetArrayItem` (`self.LineDuration`) (`self.CurrentLine`)))
      (bind _result (`/Engine/EditorBlueprintResources/StandardMacros.IncrementInt` (`self.CurrentLine`))
        (:`  `
          (if (> _result (`KismetArrayLibrary.Array_Length` (`self.Lines`)))
            (for _array_element (`self.ObjectToActive`)
              (`/Engine/EditorBlueprintResources/StandardMacros.IsValid` _array_element
                (:`Is Valid`
                  (message `/Game/VRLocomotionTemplate/Core/Interactables/Environment/I_Activate.Trigger_1` _array_element))))
            (`AudioComponent.Stop` _soundref)
            (`KismetSystemLibrary.Delay` 0.2)
            (`ActorComponent.K2_DestroyComponent` _soundref)
            (`self.K2_DestroyActor`)
            (else
              (`SceneComponent.SetVisibility` (`self.TextRender`) false false)
              (`AudioComponent.SetVolumeMultiplier` (`self.SoundRef`) 0.0)
              (`KismetSystemLibrary.Delay` 0.5)
              (`SceneComponent.SetVisibility` (`self.TextRender`) true false)
              (`AudioComponent.SetVolumeMultiplier` (`self.SoundRef`) (`/Game/VRLocomotionTemplate/Core/GameModes/BP_VRGamemode.GameVolume` (`self.Gamemode`)))))))
      (else
        (set `self.CurrentCooldown` (- (`self.CurrentCooldown`) DeltaSeconds))))))

(event `/Game/VRLocomotionTemplate/Core/Interactables/Environment/I_Activate.Trigger_1`
  (`KismetSystemLibrary.Delay` (`self.StartDelay`))
  (set `self.Active` true)
  (bind _returnvalue (`GameplayStatics.SpawnSoundAtLocation` "/Game/VRLocomotionTemplate/Audio/DemonicVoice_Cue.DemonicVoice_Cue" (`self.K2_GetActorLocation`) (struct) (`/Game/VRLocomotionTemplate/Core/GameModes/BP_VRGamemode.GameVolume` (`self.Gamemode`)) 1.0 0.0 "/Game/VRLocomotionTemplate/Audio/Attenuations/AT_Footstep.AT_Footstep" null))
  (set `self.SoundRef` _returnvalue))

(fn `UserConstructionScript`
  (`TextRenderComponent.SetWorldSize` (`self.TextRender`) (`self.TextSize`)))