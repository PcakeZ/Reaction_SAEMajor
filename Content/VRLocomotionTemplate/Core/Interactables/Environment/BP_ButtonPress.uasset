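; One-shot VR button that triggers a target object through its collision box.
; BeginPlay caches the BP_PlayerPawn reference.
; On box overlap, it compares the event's OverlappedComponent (not OtherComp) against the pawn's Cube and Cube1 components.
; A match sends Trigger1Message to TagetObject and sets Used to block further presses.
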(event `self.ReceiveBeginPlay`
  (bind _asbp_player_pawn (cast `/Game/VRLocomotionTemplate/Core/Characters/BP_PlayerPawn` (`GameplayStatics.GetPlayerPawn` 0)))
  (set `self.Player` _asbp_player_pawn))

(event `self.Box.OnComponentBeginOverlap`
  (params (OverlappedComponent :type "PrimitiveComponent Object Reference") (OtherActor :type "Actor Object Reference") (OtherComp :type "PrimitiveComponent Object Reference") (OtherBodyIndex :type Integer) (bFromSweep :type Boolean) (SweepResult :type "HitResult Structure (by ref)"))
  (bind _player (`self.Player`))
  (if (and (not (`self.Used`)) (or (== OverlappedComponent (`/Game/VRLocomotionTemplate/Core/Characters/BP_PlayerPawn.Cube` _player)) (== OverlappedComponent (`/Game/VRLocomotionTemplate/Core/Characters/BP_PlayerPawn.Cube1` _player))))
    (message `/Game/VRLocomotionTemplate/Core/Interactables/Environment/I_Activate.Trigger_1` (`self.TagetObject`))
    (set `self.Used` true)))

(fn `UserConstructionScript`)