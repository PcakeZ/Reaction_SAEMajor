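; BP_ButtonEnd is the game-ending button, usable once by the player pawn or a BP_Clone.
; BeginPlay starts dark atmosphere music, which Tick scales louder as the player's camera nears the button.
; Tick also polls the box for overlaps, then swaps the button meshes and triggers the target object.
; The press plays the end sequence at full music volume, changes camera post-processing and opens the menu level after a delay.
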(event `self.ReceiveBeginPlay`
  (bind _asbp_player_pawn (cast `/Game/VRLocomotionTemplate/Core/Characters/BP_PlayerPawn` (`GameplayStatics.GetPlayerPawn` 0)))
  (set `self.Player` _asbp_player_pawn)
  (bind _asbp_vrgamemode (cast `/Game/VRLocomotionTemplate/Core/GameModes/BP_VRGamemode` (`GameplayStatics.GetGameMode`)))
  (bind _output_get (set `self.Gamemode` _asbp_vrgamemode))
  (bind _returnvalue (`GameplayStatics.SpawnSoundAtLocation` "/Game/VRLocomotionTemplate/Audio/SoundFiles/Music/Atmos_Dark.Atmos_Dark" (`SceneComponent.K2_GetComponentLocation` (`self.Cube`)) (struct) (`/Game/VRLocomotionTemplate/Core/GameModes/BP_VRGamemode.GameVolume` _output_get) 0.1 0.0 "/Game/VRLocomotionTemplate/Audio/Attenuations/AT_DarkAtom.AT_DarkAtom" null false))
  (set `self.MusicRef` _returnvalue))

(event `self.ReceiveTick`
  (params (DeltaSeconds :type "Float (single-precision)"))
  (bind _box (`self.Box`))
  (if (not (`self.Used`))
    (`AudioComponent.SetVolumeMultiplier` (`self.MusicRef`) (* (`/Game/VRLocomotionTemplate/Core/GameModes/BP_VRGamemode.GameVolume` (`self.Gamemode`)) (/ (- (`self.HearMusicMax`) (`KismetMathLibrary.FClamp` (`KismetMathLibrary.Vector_Distance` (`SceneComponent.K2_GetComponentLocation` (`/Game/VRLocomotionTemplate/Core/Characters/BP_PlayerPawn.Camera` (`self.Player`))) (`SceneComponent.K2_GetComponentLocation` (`self.Cube2`))) 0.0 (`self.HearMusicMax`))) (`self.HearMusicMax`))))
    (if (> (+ (`KismetArrayLibrary.Array_Length` (`PrimitiveComponent.GetOverlappingActors` _box "/Game/VRLocomotionTemplate/Core/Characters/BP_PlayerPawn.BP_PlayerPawn_C")) (`KismetArrayLibrary.Array_Length` (`PrimitiveComponent.GetOverlappingActors` _box "/Game/VRLocomotionTemplate/Core/Characters/BP_Clone.BP_Clone_C"))) 0)
      (`SceneComponent.SetVisibility` (`self.Cube2`) true false)
      (`SceneComponent.SetVisibility` (`self.Cube`) false false)
      (set `self.Used` true)
      (`GameplayStatics.PlaySoundAtLocation` "/Game/VRLocomotionTemplate/Audio/SoundFiles/QA1/Applied/35_R_ButtonPress_M_V2_RO.35_R_ButtonPress_M_V2_RO" (`SceneComponent.K2_GetComponentLocation` (`self.Cube`)) (struct) (* (`/Game/VRLocomotionTemplate/Core/GameModes/BP_VRGamemode.GameVolume` (`self.Gamemode`)) 0.4) (`GameplayStatics.GetWorldDeltaSeconds`) 0.0 "/Game/VRLocomotionTemplate/Audio/Attenuations/AT_Footstep.AT_Footstep" null null)
      (message `/Game/VRLocomotionTemplate/Core/Interactables/Environment/I_Activate.Trigger_1` (`self.TagetObject`))
      (bind (_outactor _returnvalue) (`LevelSequencePlayer.CreateLevelSequencePlayer` "/Game/VRLocomotionTemplate/Core/End_Sequence.End_Sequence"))
      (`MovieSceneSequencePlayer.Play` _returnvalue)
      (`AudioComponent.SetVolumeMultiplier` (`self.MusicRef`) (`/Game/VRLocomotionTemplate/Core/GameModes/BP_VRGamemode.GameVolume` (`self.Gamemode`)))
      (set `CameraComponent.PostProcessSettings` (make `PostProcessSettings` :`SceneFringeIntensity` 2.0) (`/Game/VRLocomotionTemplate/Core/Characters/BP_PlayerPawn.Camera` (`self.Player`)))
      (`KismetSystemLibrary.Delay` 8.0)
      (`GameplayStatics.OpenLevel` "Level_Menu"))))

(fn `UserConstructionScript`)