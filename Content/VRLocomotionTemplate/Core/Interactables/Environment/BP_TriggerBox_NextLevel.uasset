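; BP_TriggerBox_NextLevel is a trigger volume in the VR locomotion template that moves the player to the next level.
; On BeginPlay it caches the player pawn as BP_PlayerPawn.
; When that pawn overlaps the box, it waits a short delay, then opens the hard-coded Level_Map_02; a Triggered flag gates this but is never set here.
; The construction script sizes the box from the BoxExtent variable.
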(event `self.ReceiveBeginPlay`
  (bind _asbp_player_pawn (cast `/Game/VRLocomotionTemplate/Core/Characters/BP_PlayerPawn` (`GameplayStatics.GetPlayerPawn` 0)))
  (set `self.Player` _asbp_player_pawn))

(event `self.Box.OnComponentBeginOverlap`
  (params (OverlappedComponent :type "PrimitiveComponent Object Reference") (OtherActor :type "Actor Object Reference") (OtherComp :type "PrimitiveComponent Object Reference") (OtherBodyIndex :type Integer) (bFromSweep :type Boolean) (SweepResult :type "HitResult Structure (by ref)"))
  (if (`self.Triggered`)
    _
    (elif (== OtherActor (`self.Player`))
      (`KismetSystemLibrary.Delay` 5.0)
      (`GameplayStatics.OpenLevel` "Level_Map_02"))))

(fn `UserConstructionScript`
  (`BoxComponent.SetBoxExtent` (`self.Box`) (`self.BoxExtent`) true))