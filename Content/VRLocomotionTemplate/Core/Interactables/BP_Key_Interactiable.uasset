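; BP_Key_Interactiable is a key object for VR that can be highlighted, picked up and launched.
; Hover events toggle custom depth on its Cube, using different stencil values for interact and grab hover.
; Interacting disables physics and attaches it to the hand; ending interaction restores physics and detaches, and ending hover also detaches.
; Grabbing applies a supplied launch impulse, with a timed Moving flag blocking repeat launches.
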(event `/Game/VRLocomotionTemplate/Core/Interactables/I_Interactable.StartHover`
  (bind _cube (`self.Cube`))
  ;[1 1 1] Highlight Object
  (`PrimitiveComponent.SetRenderCustomDepth` _cube true)
  (`PrimitiveComponent.SetCustomDepthStencilValue` _cube 2))

(event `/Game/VRLocomotionTemplate/Core/Interactables/I_Interactable.EndHover`
  ;[1 1 1] Highlight Object
  (`PrimitiveComponent.SetRenderCustomDepth` (`self.Cube`) false)
  (`self.K2_DetachFromActor` "KeepWorld" "KeepWorld" "KeepWorld"))

(event `/Game/VRLocomotionTemplate/Core/Interactables/I_Interactable.StartInteract`
  (params (Hand :type "SceneComponent Object Reference") (GunPos :type "SceneComponent Object Reference"))
  ;[1 1 1] Pickup Object
  (`PrimitiveComponent.SetSimulatePhysics` (`self.Cube`) false)
  (`self.K2_AttachToComponent` Hand "None" "KeepWorld" "KeepWorld" "KeepWorld"))

(event `/Game/VRLocomotionTemplate/Core/Interactables/I_Interactable.EndInteract`
  ;[1 1 1] Pickup Object
  (`PrimitiveComponent.SetSimulatePhysics` (`self.Cube`) true)
  (`self.K2_DetachFromActor` "KeepWorld" "KeepWorld" "KeepWorld"))

(event `/Game/VRLocomotionTemplate/Core/Interactables/I_ForceGrab.StartGrab`
  (params (LaunchVelocity :type "Vector Structure") (Time :type "Float (single-precision)"))
  (if (not (`self.Moving`))
    (`PrimitiveComponent.AddImpulse` (`self.Cube`) LaunchVelocity "None" true)
    (set `self.Moving` true)
    (`KismetSystemLibrary.Delay` Time)
    (set `self.Moving` false)))

(event `/Game/VRLocomotionTemplate/Core/Interactables/I_ForceGrab.EndGrab`)

(event `/Game/VRLocomotionTemplate/Core/Interactables/I_ForceGrab.StartGrabHover`
  (bind _cube (`self.Cube`))
  (`PrimitiveComponent.SetRenderCustomDepth` _cube true)
  (`PrimitiveComponent.SetCustomDepthStencilValue` _cube 3))

(event `/Game/VRLocomotionTemplate/Core/Interactables/I_ForceGrab.EndGrabHover`
  (`PrimitiveComponent.SetRenderCustomDepth` (`self.Cube`) false))

(fn `UserConstructionScript`)