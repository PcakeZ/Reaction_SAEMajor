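; BP_Clone is a VR player clone that replays recorded head, hand, trigger and held-object samples.
; BP_VRGamemode's read and play sample events drive LoadData playback, spawning copies of held items and forwarding trigger use through interaction messages.
; Tick lerps head and hands toward sampled transforms to smooth motion.
; The clone is destroyed on any damage or past replay length, taking held items along; its hover and force-grab helpers are never called here.
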(event `self.ReceiveAnyDamage`
  (params (Damage :type "Float (single-precision)") (DamageType :type "DamageType Object Reference") (InstigatedBy :type "Controller Object Reference") (DamageCauser :type "Actor Object Reference"))
  (`self.K2_DestroyActor` self))

(event `self.ReceiveBeginPlay`
  (bind _gamemode (`self.Gamemode`))
  ;[1 1 1] Begin Play
  (bind _asbp_vrgamemode (cast `/Game/VRLocomotionTemplate/Core/GameModes/BP_VRGamemode` (`GameplayStatics.GetGameMode`)))
  (set `self.Gamemode` _asbp_vrgamemode)
  (add `/Game/VRLocomotionTemplate/Core/GameModes/BP_VRGamemode.ReadSample` _gamemode (delegate `ReadSample`))
  (add `/Game/VRLocomotionTemplate/Core/GameModes/BP_VRGamemode.PlaySample` _gamemode (delegate `PlaySample`)))

(event `RecordingChange`
  (params (isRecording :type Boolean)))

(event `PlaySample`
  (bind _rhandobject (`self.RHandObject`))
  (bind _lhandobject (`self.LHandObject`))
  (bind (_output_headtrans _output_lhandtrans _output_rhandtrans _output_lhandobject _output_rhandobject _output_ltrigger _output_rtrigger) (break `/Game/VRLocomotionTemplate/Core/Data/Struct_PlayerInfo` (`|GetArrayItem` (`self.LoadData`) (`self.iCurrentSample`))))
  (bind _returnvalue (!= (`KismetSystemLibrary.IsValid` _output_rhandobject) (`self.RHolding`)))
  (bind _returnvalue_2 (!= (`KismetSystemLibrary.IsValid` _output_lhandobject) (`self.LHolding`)))
  (`/Engine/EditorBlueprintResources/StandardMacros.IncrementInt` (`self.iCurrentSample`)
    (:`  `
      (`/Engine/EditorBlueprintResources/StandardMacros.IncrementInt` (`self.timeOffset`)
        (:`  `
          (set `self.SampleIsRead` false)
          ;[1 1 1] Record Player Samples
          (`|ExecutionSequence` :!label _label
            (:`then_0`
              (set `self.HeadTran` _output_headtrans)
              (set `self.LHandTran` _output_lhandtrans)
              (set `self.RHandTran` _output_rhandtrans))
            (:`then_1`
              ;[1 1 1] Inputs
              (if (!= _output_ltrigger (`self.TriggerDown_L`))
                (if _output_ltrigger
                  ;;[1 1 1] Interacting with objects
                  (set `self.TriggerDown_L` true)
                  (`/Engine/EditorBlueprintResources/StandardMacros.IsValid` _lhandobject
                    (:`Is Valid`
                      (message `/Game/VRLocomotionTemplate/Core/Interactables/I_Interactable.StartUse` _lhandobject)))
                  (else
                    (set `self.TriggerDown_L` false)
                    (`/Engine/EditorBlueprintResources/StandardMacros.IsValid` _lhandobject
                      (:`Is Valid`
                        (message `/Game/VRLocomotionTemplate/Core/Interactables/I_Interactable.EndUse` _lhandobject)))))))
            (:`then_2`
              (if (!= _output_rtrigger (`self.TriggerDown_R`))
                (if _output_rtrigger
                  ;;[1 1 1] Interacting with objects
                  (set `self.TriggerDown_R` true)
                  (`/Engine/EditorBlueprintResources/StandardMacros.IsValid` _rhandobject
                    (:`Is Valid`
                      (message `/Game/VRLocomotionTemplate/Core/Interactables/I_Interactable.StartUse` _rhandobject)))
                  (else
                    (set `self.TriggerDown_R` false)
                    (`/Engine/EditorBlueprintResources/StandardMacros.IsValid` _rhandobject
                      (:`Is Valid`
                        (message `/Game/VRLocomotionTemplate/Core/Interactables/I_Interactable.EndUse` _rhandobject)))))))
            (:`then_3`
              (`/Engine/EditorBlueprintResources/StandardMacros.IsValid` _output_lhandobject
                (:`Is Valid`
                  (if _returnvalue_2
                    (bind _returnvalue_3 (`|SpawnActorFromClass` (`GameplayStatics.GetObjectClass` _output_lhandobject) (`self.LHandTran`) "Undefined" "OverrideRootScale" null null))
                    (bind _output_get (set `self.LHandObject` _returnvalue_3))
                    (message `/Game/VRLocomotionTemplate/Core/Interactables/I_Interactable.StartInteract` _output_get (`self.HandCollision_L`) (`self.GunPostion_L`))
                    (set `self.LHolding` true)
                    (`SceneComponent.SetVisibility` (`self.HandCube_L`) false false)))
                (:`Is Not Valid`
                  (if _returnvalue_2
                    (`self.K2_DestroyActor` (`self.LHandObject`))
                    (set `self.LHolding` false)
                    (`SceneComponent.SetVisibility` (`self.HandCube_L`) true false)))))
            (:`then_4`
              (`/Engine/EditorBlueprintResources/StandardMacros.IsValid` _output_rhandobject
                (:`Is Valid`
                  (if _returnvalue
                    (bind _returnvalue_4 (`|SpawnActorFromClass` (`GameplayStatics.GetObjectClass` _output_rhandobject) (`self.RHandTran`) "Undefined" "OverrideRootScale" null null))
                    (bind _output_get_2 (set `self.RHandObject` _returnvalue_4))
                    (message `/Game/VRLocomotionTemplate/Core/Interactables/I_Interactable.StartInteract` _output_get_2 (`self.LerpedHand_R`) (`self.GunPostion_R`))
                    (set `self.RHolding` true)
                    (`SceneComponent.SetVisibility` (`self.HandCube_R`) false false)))
                (:`Is Not Valid`
                  (if _returnvalue
                    (`self.K2_DestroyActor` (`self.RHandObject`))
                    (set `self.RHolding` false)
                    (`SceneComponent.SetVisibility` (`self.HandCube_R`) false false)))))
            (:`then_5`
              (if (> (`self.iCurrentSample`) (`/Game/VRLocomotionTemplate/Core/GameModes/BP_VRGamemode.ReplayLength` (`self.Gamemode`)))
                (`self.K2_DestroyActor`)))))))))

(event `ReadSample`
  (params (Sample :type Integer))
  (bind _timeoffset (`self.timeOffset`))
  (bind _replaylength (`/Game/VRLocomotionTemplate/Core/GameModes/BP_VRGamemode.ReplayLength` (`self.Gamemode`)))
  (set `self.SampleIsRead` true)
  (if (> _timeoffset _replaylength)
    (set `self.iCurrentSample` (+ (- _timeoffset _replaylength) Sample))
    (goto _label)
    (else
      (set `self.iCurrentSample` Sample)
      (goto _label))))

(event `self.ReceiveTick`
  (params (DeltaSeconds :type "Float (single-precision)"))
  (bind (_headtran_location _headtran_rotation) (`KismetMathLibrary.BreakTransform` (`self.HeadTran`)))
  (bind (_returnvalue_location _returnvalue_rotation _returnvalue_scale) (`KismetMathLibrary.BreakTransform` (`SceneComponent.K2_GetComponentToWorld` (`self.HeadHitBox`))))
  (bind _brecording (`/Game/VRLocomotionTemplate/Core/GameModes/BP_VRGamemode.bRecording` (`self.Gamemode`)))
  ;[1 1 0] Lerp Hand Positions
  (`SceneComponent.K2_SetWorldTransform` (`self.LerpedHand_L`) (`KismetMathLibrary.TLerp` (`SceneComponent.K2_GetComponentToWorld` (`self.LerpedHand_L`)) (`self.LHandTran`) 0.3) false false)
  (`SceneComponent.K2_SetWorldTransform` (`self.LerpedHand_R`) (`KismetMathLibrary.TLerp` (`SceneComponent.K2_GetComponentToWorld` (`self.LerpedHand_R`)) (`self.RHandTran`) 0.3) false false)
  (`SceneComponent.K2_SetWorldTransform` (`self.HeadHitBox`) (`KismetMathLibrary.TLerp` (`KismetMathLibrary.MakeTransform` _returnvalue_location _returnvalue_rotation _returnvalue_scale) (`KismetMathLibrary.MakeTransform` _headtran_location _headtran_rotation _returnvalue_scale) 0.3) false false)
  (if (!= (`self.bRecordingChange`) _brecording)
    (`self.RecordingChange` _brecording)))

(event `Death`
  ;[1 1 1] Dropping Objects
)

(event `self.ReceiveDestroyed`
  ;[1 1 1] Dropping Objects
  (`self.K2_DestroyActor` (`self.LHandObject`))
  (`self.K2_DestroyActor` (`self.RHandObject`)))

(fn `Force Pickup Test`
  (params (Controller :type "SceneComponent Object Reference") (ForceGrabActor :type "Actor Object Reference"))
  (returns (HitActor :type "Actor Object Reference") (NewHit :type Boolean))
  (bind _returnvalue (`SceneComponent.K2_GetComponentLocation` Controller))
  (bind (_outhit _returnvalue_2) (`KismetSystemLibrary.LineTraceSingleForObjects` _returnvalue (+ _returnvalue (* (`SceneComponent.GetForwardVector` Controller) 1000.0)) (`|MakeArray` "ObjectTypeQuery2" :!type "EObjectTypeQuery Enum") false (`|MakeArray` self :!type "Actor Object Reference") "ForOneFrame"))
  (if _returnvalue_2
    (bind (_bblockinghit _binitialoverlap _time _distance _location _impactpoint _normal _impactnormal _physmat _hitactor) (`GameplayStatics.BreakHitResult` _outhit))
    (if (`KismetSystemLibrary.DoesImplementInterface` _hitactor "/Game/VRLocomotionTemplate/Core/Interactables/I_ForceGrab.I_ForceGrab_C")
      (if (!= _hitactor ForceGrabActor)
        (`/Engine/EditorBlueprintResources/StandardMacros.IsValid` ForceGrabActor
          (:`Is Valid`
            (message `/Game/VRLocomotionTemplate/Core/Interactables/I_ForceGrab.EndGrabHover` ForceGrabActor))
          (:`Is Not Valid`
            _))
        (return _hitactor true)))
    (else
      (`/Engine/EditorBlueprintResources/StandardMacros.IsValid` ForceGrabActor
        (:`Is Valid`
          (message `/Game/VRLocomotionTemplate/Core/Interactables/I_ForceGrab.EndGrabHover` ForceGrabActor)
          (return null true))))))

(fn `ForcePickup`
  (params (SelectedActor :type "Actor Object Reference") (HandRef :type "SceneComponent Object Reference"))
  (bind (_returnvalue_x _returnvalue_y _returnvalue_z) (`KismetMathLibrary.BreakVector` (`SceneComponent.K2_GetComponentLocation` HandRef)))
  (bind (_returnvalue_x_2 _returnvalue_y_2 _returnvalue_z_2) (`KismetMathLibrary.BreakVector` (`self.K2_GetActorLocation` SelectedActor)))
  (bind _returnvalue (`KismetMathLibrary.TLerp` (`KismetMathLibrary.MakeTransform` (`KismetMathLibrary.MakeVector` _returnvalue_x_2 _returnvalue_y_2) (`self.K2_GetActorRotation` SelectedActor)) (`KismetMathLibrary.MakeTransform` (`KismetMathLibrary.MakeVector` _returnvalue_x _returnvalue_y) (`SceneComponent.K2_GetComponentRotation` HandRef)) 0.025 "EulerInterp"))
  (`self.K2_SetActorLocationAndRotation` SelectedActor (`KismetMathLibrary.MakeVector` (.x (.location _returnvalue)) (.y (.location _returnvalue)) (`KismetMathLibrary.Lerp` _returnvalue_z_2 _returnvalue_z 0.05)) (.rotation _returnvalue) false false))

(fn `HandCollisions`
  (params (InteractingActor :type "Actor Object Reference") (HandCollisionRef :type "SphereComponent Object Reference") (OtherHandInteract :type "Actor Object Reference"))
  (returns (NewActor :type "Actor Object Reference") (New :type Boolean))
  (locals (OverlappingActor :type "Actor Object Reference") (Distance :type "Float (double-precision)" :default 99999.0))
  (bind _overlappingactor (`local.OverlappingActor`))
  ;[1 1 1] Get actor closest to hand collision
  (for _array_element (`PrimitiveComponent.GetOverlappingActors` HandCollisionRef null)
    (if (and (!= _array_element self) (!= _array_element OtherHandInteract) (`KismetSystemLibrary.DoesImplementInterface` _array_element "/Game/VRLocomotionTemplate/Core/Interactables/I_Interactable.I_Interactable_C"))
      (if (< (`KismetMathLibrary.Vector_Distance` (`SceneComponent.K2_GetComponentLocation` HandCollisionRef) (`self.K2_GetActorLocation` _array_element)) (`local.Distance`))
        (set `local.OverlappingActor` _array_element))))
  ;[1 1 1] Set interacting actor based on results
  (`/Engine/EditorBlueprintResources/StandardMacros.IsValid` _overlappingactor
    (:`Is Valid`
      (`/Engine/EditorBlueprintResources/StandardMacros.IsValid` InteractingActor
        (:`Is Valid`
          (if (!= _overlappingactor InteractingActor)
            (message `/Game/VRLocomotionTemplate/Core/Interactables/I_Interactable.EndHover` InteractingActor)
            (return _overlappingactor true)))
        (:`Is Not Valid`
          (return _overlappingactor true))))
    (:`Is Not Valid`
      (`/Engine/EditorBlueprintResources/StandardMacros.IsValid` InteractingActor
        (:`Is Valid`
          (message `/Game/VRLocomotionTemplate/Core/Interactables/I_Interactable.EndHover` InteractingActor)
          (return null true))))))

(fn `UserConstructionScript`)

(fn `VelocityToPoint`
  (params (TargetPos :type "Vector Structure") (ArcHeight :type "Float (double-precision)") (Gravity :type "Float (double-precision)") (HandRef :type "SceneComponent Object Reference"))
  (returns (LaunchVel :type "Vector Structure") (Time :type "Float (double-precision)"))
  (bind (_returnvalue_x _returnvalue_y _returnvalue_z) (`KismetMathLibrary.BreakVector` (`SceneComponent.K2_GetComponentLocation` HandRef)))
  (bind _returnvalue (+ (`KismetMathLibrary.Sqrt` (/ (* 2.0 (- (- _returnvalue_z (.z TargetPos)) ArcHeight)) Gravity)) (`KismetMathLibrary.Sqrt` (/ (* -2.0 ArcHeight) Gravity))))
  (return (+ (/ (`KismetMathLibrary.MakeVector` (- _returnvalue_x (.x TargetPos)) (- _returnvalue_y (.y TargetPos))) _returnvalue) (* (* (`self.GetActorUpVector` self) (`KismetMathLibrary.Sqrt` (* (* -2.0 Gravity) ArcHeight))) (* (`KismetMathLibrary.SignOfFloat` Gravity) -1.0))) _returnvalue))