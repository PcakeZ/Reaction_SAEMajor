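; VR player pawn with teleport (navmesh-projected arc, optional tween) or continuous locomotion via a head-tracking collision body.
; Lerped hands hover, grab and use I_Interactable actors, and line-trace I_ForceGrab objects to launch them along computed arcs toward the hand.
; The gamemode drives a rolling buffer of head and hand samples.
; Death, triggered by right grip, passes samples to a BP_Clone, freezes time and enables left-stick replay scrubbing.
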(event `self.ReceiveBeginPlay`
  (bind (_relativelocation_x _relativelocation_y) (`KismetMathLibrary.BreakVector` (`SceneComponent.RelativeLocation` (`self.Camera`))))
  ;[1 1 1] Begin Play
  (bind _asbp_vrgamemode (cast `/Game/VRLocomotionTemplate/Core/GameModes/BP_VRGamemode` (`GameplayStatics.GetGameMode`)))
  (set `self.Gamemode` _asbp_vrgamemode)
  ;;[1 1 1] Centers player position regardless of position in playspace
  (`KismetSystemLibrary.Delay` 0.2)
  (`self.K2_SetActorLocation` (- (`self.K2_GetActorLocation`) (`KismetMathLibrary.MakeVector` _relativelocation_x _relativelocation_y)))
  (add `/Game/VRLocomotionTemplate/Core/GameModes/BP_VRGamemode.RecordSample` (`self.Gamemode`) (delegate `RecordSample`)))

(event `RecordSample`
  ;[1 1 1] Record Player Samples
  (if (> (`KismetArrayLibrary.Array_Length` (`self.SavedSamples`)) (`KismetMathLibrary.FTrunc` (`/Game/VRLocomotionTemplate/Core/GameModes/BP_VRGamemode.RecordTime` (`self.Gamemode`))))
    (`KismetArrayLibrary.Array_Remove` (`self.SavedSamples`)))
  (`KismetArrayLibrary.Array_Add` (`self.SavedSamples`) (make `/Game/VRLocomotionTemplate/Core/Data/Struct_PlayerInfo` (`SceneComponent.K2_GetComponentToWorld` (`self.Camera`)) (`SceneComponent.K2_GetComponentToWorld` (`self.LerpedHand_L`)) (`SceneComponent.K2_GetComponentToWorld` (`self.LerpedHand_R`)) (`self.InteractingActor_LHand`) (`self.InteractingActor_RHand`) (`self.TriggerDown_L`) (`self.TriggerDown_R`))))

(event `InputAction|JoyStickPressed_L`
  (params (Key :type "Key Structure"))
  (bind _movementtype (`self.MovementType`))
  (bind (_relativelocation_x _relativelocation_y) (`KismetMathLibrary.BreakVector` (`SceneComponent.RelativeLocation` (`self.Camera`))))
  (bind (_relativelocation_x_2 _relativelocation_y_2) (`KismetMathLibrary.BreakVector` (`SceneComponent.RelativeLocation` (`self.Camera`))))
  ;[1 1 1] Inputs
  ;;[1 1 1] Teleporting
  (:`Pressed`
    (set `self.bJoystickPressed` true)
    (switch `/Game/VRLocomotionTemplate/Core/Characters/PlayerEnums/Enum_MovementType` _movementtype
      (:`NewEnumerator0`
        (set `self.ProjectedLocation` (+ (`self.K2_GetActorLocation`) (`KismetMathLibrary.MakeVector` _relativelocation_x _relativelocation_y))))
      (:`NewEnumerator1`
        (`PrimitiveComponent.SetEnableGravity` (`self.EnvironmentCollisions`) true))))
  (:`Released`
    (set `self.bJoystickPressed` false)
    (switch `/Game/VRLocomotionTemplate/Core/Characters/PlayerEnums/Enum_MovementType` _movementtype
      (:`NewEnumerator0`
        (if (`self.bTPTween`)
          (set `self.bIsTweening` true)
          (else
            (`self.K2_SetActorLocation` (- (`self.ProjectedLocation`) (`KismetMathLibrary.MakeVector` _relativelocation_x_2 _relativelocation_y_2))))))
      (:`NewEnumerator1`
        (`PrimitiveComponent.SetEnableGravity` (`self.EnvironmentCollisions`) false)))))

(event `self.ReceiveTick`
  (params (DeltaSeconds :type "Float (single-precision)"))
  (bind _returnvalue (`self.K2_GetActorLocation`))
  (bind (_returnvalue_x _returnvalue_y _returnvalue_z) (`KismetMathLibrary.BreakVector` (`self.K2_GetActorLocation`)))
  (bind _returnvalue_2 (`self.GetInputAxisValue`))
  (bind _gamemode (`self.Gamemode`))
  (bind (_returnvalue_x_2 _returnvalue_y_2) (`KismetMathLibrary.BreakVector` (`SceneComponent.K2_GetComponentLocation` (`self.Camera`))))
  (bind (_relativelocation_x _relativelocation_y) (`KismetMathLibrary.BreakVector` (`SceneComponent.RelativeLocation` (`self.Camera`))))
  (bind _returnvalue_3 (- (`self.ProjectedLocation`) (`KismetMathLibrary.MakeVector` _relativelocation_x _relativelocation_y)))
  ;[1 1 1] Tick
  (`|ExecutionSequence`
    (:`then_0`
      ;;[1 1 1] Keeps track of collision - similar to half-life
      (if (not (`self.bJoystickPressed`))
        (`SceneComponent.K2_SetWorldLocation` (`self.LocomotionCollisions`) (`KismetMathLibrary.MakeVector` _returnvalue_x_2 _returnvalue_y_2 (+ _returnvalue_z 92.0)) false false)
        (`self.MoveCollisions`)))
    (:`then_1`
      ;;[1 1 1] Movement
      (switch `/Game/VRLocomotionTemplate/Core/Characters/PlayerEnums/Enum_MovementType` (`self.MovementType`)
        (:`NewEnumerator0`
          ;;;[1 1 1] Teleport
          (if (`self.bJoystickPressed`)
            (bind (_projectedlocation _vaildlocation) (`self.FindTeleportLocation`))
            (if _vaildlocation
              (set `self.ProjectedLocation` _projectedlocation))
            (elif (`self.bTPTween`)
              ;;;;[1 1 1] Tween Teleport
              (if (`self.bIsTweening`)
                (if (> (`KismetMathLibrary.Vector_Distance` _returnvalue_3 _returnvalue) 20.0)
                  (`self.K2_SetActorLocation` (`KismetMathLibrary.VLerp` _returnvalue_3 _returnvalue 0.7))
                  (else
                    (set `self.bIsTweening` false)))))))
        (:`NewEnumerator1`
          ;;;[1 1 1] Continuous Movement
          (if (`self.bJoystickPressed`)
            (if (`self.bUseHandDirection`)
              (`self.ContinuousMovement` (`self.MotionController_L`))
              (else
                (`self.ContinuousMovement` (`self.Camera`))))))))
    (:`then_2`
      ;;[1 1 1] Interacting with Objects
      (`|ExecutionSequence`
        (:`then_0`
          ;;;[1 1 1] Check Left Hand Collisions
          (if (not (`self.bGripInteraction_L`))
            (bind (_newactor _new) (`self.HandCollisions` (`self.InteractingActor_LHand`) (`self.HandCollision_L`) (`self.InteractingActor_RHand`)))
            (if _new
              (bind _output_get (set `self.InteractingActor_LHand` _newactor))
              (`/Engine/EditorBlueprintResources/StandardMacros.IsValid` _output_get
                (:`Is Valid`
                  (message `/Game/VRLocomotionTemplate/Core/Interactables/I_Interactable.StartHover` _output_get)
                  ;;;[1 1 1] Test for grabable objects when TestGrab is active
                  (if (`self.bTestGrab_L`)
                    (message `/Game/VRLocomotionTemplate/Core/Interactables/I_Interactable.StartInteract` (`self.InteractingActor_LHand`) (`self.MotionController_L`) (`self.GunPostion_L`))
                    (set `self.bGripInteraction_L` true)
                    (`SceneComponent.SetVisibility` (`self.Cube1`) false false)
                    (set `self.bTestGrab_L` false)))
                (:`Is Not Valid`
                  (if (not (`self.ForceGrabbed_L`)) :!label _label
                    ;;;[1 1 1] Force grab test
                    (bind (_hitactor _newhit) (`self.Force Pickup Test` (`self.LerpedHand_L`) (`self.ForceGrabActor_L`)))
                    (if _newhit
                      (bind _output_get_2 (set `self.ForceGrabActor_L` _hitactor))
                      (`/Engine/EditorBlueprintResources/StandardMacros.IsValid` _output_get_2
                        (:`Is Valid`
                          (message `/Game/VRLocomotionTemplate/Core/Interactables/I_ForceGrab.StartGrabHover` _output_get_2)))))))
              (else
                (`/Engine/EditorBlueprintResources/StandardMacros.IsValid` (`self.InteractingActor_LHand`)
                  (:`Is Not Valid`
                    (goto _label)))))))
        (:`then_1`
          ;;;[1 1 1] Check Right Hand Collisions
          (if (not (`self.bGripInteraction_R`))
            (bind (_newactor_2 _new_2) (`self.HandCollisions` (`self.InteractingActor_RHand`) (`self.HandCollision_R`) (`self.InteractingActor_LHand`)))
            (if _new_2
              (bind _output_get_3 (set `self.InteractingActor_RHand` _newactor_2))
              (`/Engine/EditorBlueprintResources/StandardMacros.IsValid` _output_get_3
                (:`Is Valid`
                  (message `/Game/VRLocomotionTemplate/Core/Interactables/I_Interactable.StartHover` _output_get_3)
                  ;;;[1 1 1] Test for grabable objects when TestGrab is active
                  (if (`self.bTestGrab_R`)
                    (message `/Game/VRLocomotionTemplate/Core/Interactables/I_Interactable.StartInteract` (`self.InteractingActor_RHand`) (`self.MotionController_R`) (`self.GunPostion_R`))
                    (set `self.bGripInteraction_R` true)
                    (`SceneComponent.SetVisibility` (`self.Cube`) false false)
                    (set `self.bTestGrab_R` false)))
                (:`Is Not Valid`
                  (if (not (`self.ForceGrabbed_R`)) :!label _label_2
                    ;;;[1 1 1] Force grab test
                    (bind (_hitactor_2 _newhit_2) (`self.Force Pickup Test` (`self.LerpedHand_R`) (`self.ForceGrabActor_R`)))
                    (if _newhit_2
                      (bind _output_get_4 (set `self.ForceGrabActor_R` _hitactor_2))
                      (`/Engine/EditorBlueprintResources/StandardMacros.IsValid` _output_get_4
                        (:`Is Valid`
                          (message `/Game/VRLocomotionTemplate/Core/Interactables/I_ForceGrab.StartGrabHover` _output_get_4)))))))
              (else
                (`/Engine/EditorBlueprintResources/StandardMacros.IsValid` (`self.InteractingActor_RHand`)
                  (:`Is Not Valid`
                    (goto _label_2)))))))))
    (:`then_3`
      ;;[1 1 0] Lerp Hand Positions
      (`SceneComponent.K2_SetWorldTransform` (`self.LerpedHand_L`) (`KismetMathLibrary.TLerp` (`SceneComponent.K2_GetComponentToWorld` (`self.LerpedHand_L`)) (`SceneComponent.K2_GetComponentToWorld` (`self.MotionController_L`)) (* (`GameplayStatics.GetWorldDeltaSeconds`) 20.0)) true false)
      (`SceneComponent.K2_SetWorldTransform` (`self.LerpedHand_R`) (`KismetMathLibrary.TLerp` (`SceneComponent.K2_GetComponentToWorld` (`self.LerpedHand_R`)) (`SceneComponent.K2_GetComponentToWorld` (`self.MotionController_R`)) (* (`GameplayStatics.GetWorldDeltaSeconds`) 20.0)) true false))
    (:`then_4`
      (if (and (not (`self.bJoystickPressed`)) (`self.bDead`))
        (if (!= _returnvalue_2 0.0)
          (if (> _returnvalue_2 0.0)
            (set `/Game/VRLocomotionTemplate/Core/GameModes/BP_VRGamemode.RightScrubing` true _gamemode)
            (set `/Game/VRLocomotionTemplate/Core/GameModes/BP_VRGamemode.LeftScrubing` false _gamemode)
            (else
              (set `/Game/VRLocomotionTemplate/Core/GameModes/BP_VRGamemode.LeftScrubing` true _gamemode)
              (set `/Game/VRLocomotionTemplate/Core/GameModes/BP_VRGamemode.RightScrubing` false _gamemode)))
          (else
            (set `/Game/VRLocomotionTemplate/Core/GameModes/BP_VRGamemode.RightScrubing` false _gamemode)
            (set `/Game/VRLocomotionTemplate/Core/GameModes/BP_VRGamemode.LeftScrubing` false _gamemode)))))))

(event `InputAction|MenuLeft`
  (params (Key :type "Key Structure"))
  ;[1 1 1] Restart Level
  (:`Pressed`
    (`GameplayStatics.OpenLevel` "LocomotionSandbox")))

(event `InputAction|Trigger_L`
  (params (Key :type "Key Structure"))
  (bind _bgripinteraction_l (`self.bGripInteraction_L`))
  (bind _interactingactor_lhand (`self.InteractingActor_LHand`))
  (bind _forcegrabactor_l (`self.ForceGrabActor_L`))
  (:`Pressed`
    ;[1 1 1] Inputs
    ;;[1 1 1] Interacting with objects
    (set `self.TriggerDown_L` true)
    (if _bgripinteraction_l
      (message `/Game/VRLocomotionTemplate/Core/Interactables/I_Interactable.StartUse` _interactingactor_lhand)
      (else
        ;;[1 1 1] ForceGrabbing Object
        (`/Engine/EditorBlueprintResources/StandardMacros.IsValid` _forcegrabactor_l
          (:`Is Valid`
            (bind (_launchvel _time) (`self.VelocityToPoint` (`self.K2_GetActorLocation` _forcegrabactor_l) 200.0 -980.0 (`self.LerpedHand_L`)))
            (message `/Game/VRLocomotionTemplate/Core/Interactables/I_ForceGrab.StartGrab` _forcegrabactor_l _launchvel _time))
          (:`Is Not Valid`
            _))
        (set `self.bTestGrab_L` true)
        (`KismetSystemLibrary.Delay` 1.0)
        (set `self.bTestGrab_L` false))))
  (:`Released`
    (set `self.TriggerDown_L` false)
    (if _bgripinteraction_l
      (message `/Game/VRLocomotionTemplate/Core/Interactables/I_Interactable.EndUse` _interactingactor_lhand)
      (else
        (set `self.bTestGrab_L` false)))))

(event `InputAction|Trigger_R`
  (params (Key :type "Key Structure"))
  (bind _bgripinteraction_r (`self.bGripInteraction_R`))
  (bind _interactingactor_rhand (`self.InteractingActor_RHand`))
  (bind _forcegrabactor_r (`self.ForceGrabActor_R`))
  (:`Pressed`
    ;[1 1 1] Inputs
    ;;[1 1 1] Interacting with objects
    (set `self.TriggerDown_R` true)
    (if _bgripinteraction_r
      (message `/Game/VRLocomotionTemplate/Core/Interactables/I_Interactable.StartUse` _interactingactor_rhand)
      (else
        ;;[1 1 1] ForceGrabbing Object
        (`/Engine/EditorBlueprintResources/StandardMacros.IsValid` _forcegrabactor_r
          (:`Is Valid`
            (bind (_launchvel _time) (`self.VelocityToPoint` (`self.K2_GetActorLocation` _forcegrabactor_r) 200.0 -980.0 (`self.LerpedHand_R`)))
            (message `/Game/VRLocomotionTemplate/Core/Interactables/I_ForceGrab.StartGrab` _forcegrabactor_r _launchvel _time))
          (:`Is Not Valid`
            _))
        (set `self.bTestGrab_R` true)
        (`KismetSystemLibrary.Delay` 1.0)
        (set `self.bTestGrab_R` false))))
  (:`Released`
    (set `self.TriggerDown_R` false)
    (if _bgripinteraction_r
      (message `/Game/VRLocomotionTemplate/Core/Interactables/I_Interactable.EndUse` _interactingactor_rhand)
      (else
        (set `self.bTestGrab_R` false)))))

(event `InputAction|Grip_L`
  (params (Key :type "Key Structure"))
  (bind _interactingactor_lhand (`self.InteractingActor_LHand`))
  ;[1 1 1] Inputs
  ;;[1 1 1] Dropping Objects
  (:`Released`
    (`/Engine/EditorBlueprintResources/StandardMacros.IsValid` _interactingactor_lhand
      (:`Is Valid`
        (message `/Game/VRLocomotionTemplate/Core/Interactables/I_Interactable.EndInteract` _interactingactor_lhand)
        (set `self.bGripInteraction_L` false)
        (`SceneComponent.SetVisibility` (`self.Cube1`) true false)))))

(event `InputAction|Grip_R`
  (params (Key :type "Key Structure"))
  (bind _interactingactor_rhand (`self.InteractingActor_RHand`))
  ;[1 1 1] Inputs
  ;;[1 1 1] Dropping Objects
  (:`Pressed`
    (`self.Death`))
  (:`Released`
    (`/Engine/EditorBlueprintResources/StandardMacros.IsValid` _interactingactor_rhand
      (:`Is Valid`
        (message `/Game/VRLocomotionTemplate/Core/Interactables/I_Interactable.EndInteract` _interactingactor_rhand)
        (set `self.bGripInteraction_R` false)
        (`SceneComponent.SetVisibility` (`self.Cube`) true false)))))

(event `Death`
  (bind _savedsamples (`self.SavedSamples`))
  (bind _gamemode (`self.Gamemode`))
  (bind _returnvalue (- (`KismetArrayLibrary.Array_Length` _savedsamples) 1))
  (set `self.bDead` true)
  (bind _returnvalue_2 (`|SpawnActorFromClass` "/Game/VRLocomotionTemplate/Core/Characters/BP_Clone.BP_Clone_C" (`self.GetTransform`) "AlwaysSpawn" "OverrideRootScale" null null))
  (set `/Game/VRLocomotionTemplate/Core/Characters/BP_Clone.LoadData` _savedsamples _returnvalue_2)
  (set `/Game/VRLocomotionTemplate/Core/GameModes/BP_VRGamemode.bRecording` false _gamemode)
  (set `/Game/VRLocomotionTemplate/Core/GameModes/BP_VRGamemode.ReplayLength` _returnvalue _gamemode)
  (set `/Game/VRLocomotionTemplate/Core/GameModes/BP_VRGamemode.CurrentSample` _returnvalue _gamemode)
  (`GameplayStatics.SetGlobalTimeDilation` 0.0))

(fn `ContinuousMovement`
  (params (MovementDirection :type "SceneComponent Object Reference"))
  (bind (_returnvalue_roll _returnvalue_pitch _returnvalue_yaw) (`KismetMathLibrary.BreakRotator` (`SceneComponent.K2_GetComponentRotation` MovementDirection)))
  (bind _environmentcollisions (`self.EnvironmentCollisions`))
  (bind _returnvalue (`KismetMathLibrary.MakeRotator` 0.0 0.0 _returnvalue_yaw))
  (bind _returnvalue_2 (`SceneComponent.K2_GetComponentLocation` _environmentcollisions))
  (bind (_relativelocation_x _relativelocation_y) (`KismetMathLibrary.BreakVector` (`SceneComponent.RelativeLocation` (`self.Camera`))))
  (bind _z (.z _returnvalue_2))
  (bind (_returnvalue_x _returnvalue_y) (`KismetMathLibrary.BreakVector` (+ _returnvalue_2 (* (+ (* (`KismetMathLibrary.GetRightVector` _returnvalue) (`self.GetInputAxisValue`)) (* (`KismetMathLibrary.GetForwardVector` _returnvalue) (`self.GetInputAxisValue`))) (`self.MovementSpeed`)))))
  ;[1 1 1] Moves Environment Collision, then moves actor (This ensures the player doesn't collide with anything)
  (`SceneComponent.K2_SetWorldLocation` _environmentcollisions (`KismetMathLibrary.MakeVector` _returnvalue_x _returnvalue_y _z) false false)
  (`self.K2_SetActorLocation` (- (`KismetMathLibrary.MakeVector` (.x _returnvalue_2) (.y _returnvalue_2) (- _z 92.0)) (`KismetMathLibrary.MakeVector` _relativelocation_x _relativelocation_y))))

(fn `FindTeleportLocation`
  (returns (ProjectedLocation :type "Vector Structure") (VaildLocation :type Boolean))
  (bind _motioncontroller_l (`self.MotionController_L`))
  (bind (_outhit _outpathpositions _outlasttracedestination _returnvalue) (`GameplayStatics.Blueprint_PredictProjectilePath_ByTraceChannel` (`SceneComponent.K2_GetComponentLocation` _motioncontroller_l) (* (`SceneComponent.GetForwardVector` _motioncontroller_l) (`self.TeleportArcDistance`)) true 1.0 "ECC_Visibility" true (`|MakeArray` (`self.InteractingActor_RHand`) (`self.InteractingActor_LHand`) self :!type "Actor Object Reference") "ForOneFrame"))
  (if _returnvalue
    (bind (_projectedlocation _returnvalue_2) (`NavigationSystemV1.K2_ProjectPointToNavigation` (`.Location` (`GameplayStatics.BreakHitResult` _outhit))))
    (`KismetSystemLibrary.DrawDebugCylinder` _projectedlocation (+ _projectedlocation (0.0 0.0 3.0)) 30.0 12 (struct :`R` 1.0 :`A` 1.0) 0.0 0.5)
    (return _projectedlocation _returnvalue_2)))

(fn `Force Pickup Test`
  (params (Controller :type "SceneComponent Object Reference") (ForceGrabActor :type "Actor Object Reference"))
  (returns (HitActor :type "Actor Object Reference") (NewHit :type Boolean))
  (bind _returnvalue (`SceneComponent.K2_GetComponentLocation` Controller))
  (bind (_outhit _returnvalue_2) (`KismetSystemLibrary.LineTraceSingleForObjects` _returnvalue (+ _returnvalue (* (`SceneComponent.GetForwardVector` Controller) 1000.0)) (`|MakeArray` "ObjectTypeQuery2" :!type "EObjectTypeQuery Enum") false (`|MakeArray` self :!type "Actor Object Reference") "ForOneFrame"))
  (if _returnvalue_2
    (bind (_bblockinghit _binitialoverlap _time _distance _location _impactpoint _normal _impactnormal _physmat _hitactor) (`GameplayStatics.BreakHitResult` _outhit))
    (if (`KismetSystemLibrary.DoesImplementInterface` _hitactor "/Game/VRLocomotionTemplate/Core/Interactables/I_ForceGrab.I_ForceGrab_C")
      (if (!= _hitactor ForceGrabActor)
        (`/Engine/EditorBlueprintResources/StandardMacros.IsValid` ForceGrabActor
          (:`Is Valid`
            (message `/Game/VRLocomotionTemplate/Core/Interactables/I_ForceGrab.EndGrabHover` ForceGrabActor))
          (:`Is Not Valid`
            _))
        (return _hitactor true)))
    (else
      (`/Engine/EditorBlueprintResources/StandardMacros.IsValid` ForceGrabActor
        (:`Is Valid`
          (message `/Game/VRLocomotionTemplate/Core/Interactables/I_ForceGrab.EndGrabHover` ForceGrabActor)
          (return null true))))))

(fn `ForcePickup`
  (params (SelectedActor :type "Actor Object Reference") (HandRef :type "SceneComponent Object Reference"))
  (bind (_returnvalue_x _returnvalue_y _returnvalue_z) (`KismetMathLibrary.BreakVector` (`SceneComponent.K2_GetComponentLocation` HandRef)))
  (bind (_returnvalue_x_2 _returnvalue_y_2 _returnvalue_z_2) (`KismetMathLibrary.BreakVector` (`self.K2_GetActorLocation` SelectedActor)))
  (bind _returnvalue (`KismetMathLibrary.TLerp` (`KismetMathLibrary.MakeTransform` (`KismetMathLibrary.MakeVector` _returnvalue_x_2 _returnvalue_y_2) (`self.K2_GetActorRotation` SelectedActor)) (`KismetMathLibrary.MakeTransform` (`KismetMathLibrary.MakeVector` _returnvalue_x _returnvalue_y) (`SceneComponent.K2_GetComponentRotation` HandRef)) 0.025 "EulerInterp"))
  (`self.K2_SetActorLocationAndRotation` SelectedActor (`KismetMathLibrary.MakeVector` (.x (.location _returnvalue)) (.y (.location _returnvalue)) (`KismetMathLibrary.Lerp` _returnvalue_z_2 _returnvalue_z 0.05)) (.rotation _returnvalue) false false))

(fn `HandCollisions`
  (params (InteractingActor :type "Actor Object Reference") (HandCollisionRef :type "SphereComponent Object Reference") (OtherHandInteract :type "Actor Object Reference"))
  (returns (NewActor :type "Actor Object Reference") (New :type Boolean))
  (locals (OverlappingActor :type "Actor Object Reference") (Distance :type "Float (double-precision)" :default 99999.0))
  (bind _overlappingactor (`local.OverlappingActor`))
  ;[1 1 1] Get actor closest to hand collision
  (for _array_element (`PrimitiveComponent.GetOverlappingActors` HandCollisionRef null)
    (if (and (!= _array_element self) (!= _array_element OtherHandInteract) (`KismetSystemLibrary.DoesImplementInterface` _array_element "/Game/VRLocomotionTemplate/Core/Interactables/I_Interactable.I_Interactable_C"))
      (if (< (`KismetMathLibrary.Vector_Distance` (`SceneComponent.K2_GetComponentLocation` HandCollisionRef) (`self.K2_GetActorLocation` _array_element)) (`local.Distance`))
        (set `local.OverlappingActor` _array_element))))
  ;[1 1 1] Set interacting actor based on results
  (`/Engine/EditorBlueprintResources/StandardMacros.IsValid` _overlappingactor
    (:`Is Valid`
      (`/Engine/EditorBlueprintResources/StandardMacros.IsValid` InteractingActor
        (:`Is Valid`
          (if (!= _overlappingactor InteractingActor)
            (message `/Game/VRLocomotionTemplate/Core/Interactables/I_Interactable.EndHover` InteractingActor)
            (return _overlappingactor true)))
        (:`Is Not Valid`
          (return _overlappingactor true))))
    (:`Is Not Valid`
      (`/Engine/EditorBlueprintResources/StandardMacros.IsValid` InteractingActor
        (:`Is Valid`
          (message `/Game/VRLocomotionTemplate/Core/Interactables/I_Interactable.EndHover` InteractingActor)
          (return null true))))))

(fn `MoveCollisions`
  (locals (iOverlappingObjects :type Integer))
  ;[1 1 1] Keeps track of collision - similar to half-life
  (for _array_element (`PrimitiveComponent.GetOverlappingActors` (`self.LocomotionCollisions`) null)
    (if (not (or (`KismetSystemLibrary.DoesImplementInterface` _array_element "/Game/VRLocomotionTemplate/Core/Interactables/I_Interactable.I_Interactable_C") (== _array_element self)))
      (`/Engine/EditorBlueprintResources/StandardMacros.IncrementInt` (`local.iOverlappingObjects`))))
  (if (<= (`local.iOverlappingObjects`) 0)
    (`SceneComponent.K2_SetWorldLocation` (`self.EnvironmentCollisions`) (`SceneComponent.K2_GetComponentLocation` (`self.LocomotionCollisions`)) false false)))

(fn `UserConstructionScript`)

(fn `VelocityToPoint`
  (params (TargetPos :type "Vector Structure") (ArcHeight :type "Float (double-precision)") (Gravity :type "Float (double-precision)") (HandRef :type "SceneComponent Object Reference"))
  (returns (LaunchVel :type "Vector Structure") (Time :type "Float (double-precision)"))
  (bind (_returnvalue_x _returnvalue_y _returnvalue_z) (`KismetMathLibrary.BreakVector` (`SceneComponent.K2_GetComponentLocation` HandRef)))
  (bind _returnvalue (+ (`KismetMathLibrary.Sqrt` (/ (* 2.0 (- (- _returnvalue_z (.z TargetPos)) ArcHeight)) Gravity)) (`KismetMathLibrary.Sqrt` (/ (* -2.0 ArcHeight) Gravity))))
  (return (+ (/ (`KismetMathLibrary.MakeVector` (- _returnvalue_x (.x TargetPos)) (- _returnvalue_y (.y TargetPos))) _returnvalue) (* (* (`self.GetActorUpVector` self) (`KismetMathLibrary.Sqrt` (* (* -2.0 Gravity) ArcHeight))) (* (`KismetMathLibrary.SignOfFloat` Gravity) -1.0))) _returnvalue))