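; VR shotgun actor that can be highlighted, picked up, pulled from afar and fired.
; Hover events toggle custom-depth stencil outlines, while interact events toggle physics and attach or detach it from the hand.
; Grab applies a supplied launch impulse, with a timed lock against repeats.
; Use calls Shoot, which spawns BP_Bullet pellets with impulses, rolling random spread separately for rotation and direction, then plays the shot sound.
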(event `/Game/VRLocomotionTemplate/Core/Interactables/I_Interactable.StartHover`
  (bind _staticmesh (`self.StaticMesh`))
  ;[1 1 1] Highlight Object
  (`PrimitiveComponent.SetRenderCustomDepth` _staticmesh true)
  (`PrimitiveComponent.SetCustomDepthStencilValue` _staticmesh 2))

(event `/Game/VRLocomotionTemplate/Core/Interactables/I_Interactable.EndHover`
  ;[1 1 1] Highlight Object
  (`PrimitiveComponent.SetRenderCustomDepth` (`self.StaticMesh`) false)
  (`self.K2_DetachFromActor` "KeepWorld" "KeepWorld" "KeepWorld"))

(event `/Game/VRLocomotionTemplate/Core/Interactables/I_Interactable.StartInteract`
  (params (Hand :type "SceneComponent Object Reference") (GunPos :type "SceneComponent Object Reference"))
  ;[1 1 1] Pickup Object
  (`PrimitiveComponent.SetSimulatePhysics` (`self.Gun`) false)
  (`self.K2_SetActorLocationAndRotation` (`SceneComponent.K2_GetComponentLocation` GunPos) (`SceneComponent.K2_GetComponentRotation` GunPos))
  (`self.K2_AttachToComponent` Hand "None" "KeepWorld" "KeepWorld" "KeepWorld")
  (`PrimitiveComponent.SetRenderCustomDepth` (`self.StaticMesh`) false))

(event `/Game/VRLocomotionTemplate/Core/Interactables/I_Interactable.EndInteract`
  ;[1 1 1] Pickup Object
  (`PrimitiveComponent.SetSimulatePhysics` (`self.Gun`) true)
  (`self.K2_DetachFromActor` "KeepWorld" "KeepWorld" "KeepWorld"))

(event `/Game/VRLocomotionTemplate/Core/Interactables/I_Interactable.StartUse`
  ;[1 1 1] Pickup Object
  (`self.Shoot`))

(event `/Game/VRLocomotionTemplate/Core/Interactables/I_Interactable.EndUse`
  ;[1 1 1] Pickup Object
)

(event `/Game/VRLocomotionTemplate/Core/Interactables/I_ForceGrab.StartGrab`
  (params (LaunchVelocity :type "Vector Structure") (Time :type "Float (single-precision)"))
  (if (not (`self.Moving`))
    (`PrimitiveComponent.AddImpulse` (`self.Gun`) LaunchVelocity "None" true)
    (set `self.Moving` true)
    (`KismetSystemLibrary.Delay` Time)
    (set `self.Moving` false)))

(event `/Game/VRLocomotionTemplate/Core/Interactables/I_ForceGrab.EndGrab`)

(event `/Game/VRLocomotionTemplate/Core/Interactables/I_ForceGrab.StartGrabHover`
  (bind _staticmesh (`self.StaticMesh`))
  (`PrimitiveComponent.SetRenderCustomDepth` _staticmesh true)
  (`PrimitiveComponent.SetCustomDepthStencilValue` _staticmesh 3))

(event `/Game/VRLocomotionTemplate/Core/Interactables/I_ForceGrab.EndGrabHover`
  (`PrimitiveComponent.SetRenderCustomDepth` (`self.StaticMesh`) false))

(fn `Shoot`
  (bind (_spread_x _spread_y) (`KismetMathLibrary.BreakVector2D` (`self.Spread`)))
  (bind _returnvalue (`SceneComponent.K2_GetComponentToWorld` (`self.ShootingPos`)))
  (bind _returnvalue_2 (+ (.yaw (.rotation _returnvalue)) (`KismetMathLibrary.RandomFloatInRange` (* _spread_x -1.0) _spread_x)))
  (bind _returnvalue_3 (+ (.pitch (.rotation _returnvalue)) (`KismetMathLibrary.RandomFloatInRange` (* _spread_y -1.0) _spread_y)))
  (for _ (range (+ (`self.iPellets`) 1))
    (bind _returnvalue_4 (`|SpawnActorFromClass` "/Game/VRLocomotionTemplate/Core/Weapons/BP_Bullet.BP_Bullet_C" (`KismetMathLibrary.MakeTransform` (.location _returnvalue) (`KismetMathLibrary.MakeRotator` (.roll (.rotation _returnvalue)) _returnvalue_3 _returnvalue_2) (0.03 0.015 0.015)) "Undefined" "OverrideRootScale" null null))
    (`PrimitiveComponent.AddImpulse` (`/Game/VRLocomotionTemplate/Core/Weapons/BP_Bullet.Cube` _returnvalue_4) (* (`KismetMathLibrary.GetForwardVector` (`KismetMathLibrary.MakeRotator` (.roll (.rotation _returnvalue)) _returnvalue_3 _returnvalue_2)) (`self.BulletSpeed`)) "None" true))
  (`GameplayStatics.PlaySoundAtLocation` "/Game/VRLocomotionTemplate/Audio/SoundFiles/Weapon/6_Shotgun_Shot_M_V1_RO.6_Shotgun_Shot_M_V1_RO" (`SceneComponent.K2_GetComponentLocation` (`self.ShootingPos`)) (struct) 1.0 1.0 0.0 null null null))

(fn `UserConstructionScript`)