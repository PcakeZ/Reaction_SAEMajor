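; BP_Pistol is a VR pistol that can be highlighted, picked up, launched by a grab and fired.
; Hover and grab-hover outline it with different custom depth stencil values, while interaction toggles physics and attaches it to or detaches it from the hand.
; Grab applies a supplied velocity impulse, locked out for the given time.
; Use calls Shoot, which spawns an impulse-driven BP_Bullet at the muzzle and plays a bang.
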(event `/Game/VRLocomotionTemplate/Core/Interactables/I_Interactable.StartHover`
  (bind _gun (`self.Gun`))
  ;[1 1 1] Highlight Object
  (`PrimitiveComponent.SetRenderCustomDepth` _gun true)
  (`PrimitiveComponent.SetCustomDepthStencilValue` _gun 2))

(event `/Game/VRLocomotionTemplate/Core/Interactables/I_Interactable.EndHover`
  ;[1 1 1] Highlight Object
  (`PrimitiveComponent.SetRenderCustomDepth` (`self.Gun`) false)
  (`self.K2_DetachFromActor` "KeepWorld" "KeepWorld" "KeepWorld"))

(event `/Game/VRLocomotionTemplate/Core/Interactables/I_Interactable.StartInteract`
  (params (Hand :type "SceneComponent Object Reference") (GunPos :type "SceneComponent Object Reference"))
  ;[1 1 1] Pickup Object
  (`PrimitiveComponent.SetSimulatePhysics` (`self.Gun`) false)
  (`self.K2_SetActorLocationAndRotation` (`SceneComponent.K2_GetComponentLocation` GunPos) (`SceneComponent.K2_GetComponentRotation` GunPos))
  (`self.K2_AttachToComponent` Hand "None" "KeepWorld" "KeepWorld" "KeepWorld")
  (`PrimitiveComponent.SetRenderCustomDepth` (`self.Gun`) false))

(event `/Game/VRLocomotionTemplate/Core/Interactables/I_Interactable.EndInteract`
  ;[1 1 1] Pickup Object
  (`PrimitiveComponent.SetSimulatePhysics` (`self.Gun`) true)
  (`self.K2_DetachFromActor` "KeepWorld" "KeepWorld" "KeepWorld"))

(event `/Game/VRLocomotionTemplate/Core/Interactables/I_Interactable.StartUse`
  ;[1 1 1] Pickup Object
  (`self.Shoot`))

(event `/Game/VRLocomotionTemplate/Core/Interactables/I_Interactable.EndUse`
  ;[1 1 1] Pickup Object
)

(event `/Game/VRLocomotionTemplate/Core/Interactables/I_ForceGrab.StartGrab`
  (params (LaunchVelocity :type "Vector Structure") (Time :type "Float (single-precision)"))
  (if (not (`self.Moving`))
    (`PrimitiveComponent.AddImpulse` (`self.Gun`) LaunchVelocity "None" true)
    (set `self.Moving` true)
    (`KismetSystemLibrary.Delay` Time)
    (set `self.Moving` false)))

(event `/Game/VRLocomotionTemplate/Core/Interactables/I_ForceGrab.EndGrab`)

(event `/Game/VRLocomotionTemplate/Core/Interactables/I_ForceGrab.StartGrabHover`
  (bind _gun (`self.Gun`))
  (`PrimitiveComponent.SetRenderCustomDepth` _gun true)
  (`PrimitiveComponent.SetCustomDepthStencilValue` _gun 3))

(event `/Game/VRLocomotionTemplate/Core/Interactables/I_ForceGrab.EndGrabHover`
  (`PrimitiveComponent.SetRenderCustomDepth` (`self.Gun`) false))

(fn `Shoot`
  (bind (_returnvalue_location _returnvalue_rotation) (`KismetMathLibrary.BreakTransform` (`SceneComponent.K2_GetComponentToWorld` (`self.ShootingPos`))))
  (bind _returnvalue (`|SpawnActorFromClass` "/Game/VRLocomotionTemplate/Core/Weapons/BP_Bullet.BP_Bullet_C" (`KismetMathLibrary.MakeTransform` _returnvalue_location _returnvalue_rotation (0.03 0.015 0.015)) "Undefined" "OverrideRootScale" null null))
  (`PrimitiveComponent.AddImpulse` (`/Game/VRLocomotionTemplate/Core/Weapons/BP_Bullet.Cube` _returnvalue) (* (`SceneComponent.GetForwardVector` (`self.ShootingPos`)) (`self.BulletSpeed`)) "None" true)
  (`GameplayStatics.PlaySoundAtLocation` "/Game/VRLocomotionTemplate/Audio/S_Bang.S_Bang" (`SceneComponent.K2_GetComponentLocation` (`self.ShootingPos`)) (struct) 1.0 1.0 0.0 null null null))

(fn `UserConstructionScript`)