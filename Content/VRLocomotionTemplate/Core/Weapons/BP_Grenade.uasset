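; BP_Grenade is a timed explosive weapon actor for the VR locomotion template that detonates automatically after a fuse delay.
; BeginPlay caches the player pawn and VR game mode, then waits a short pause plus FAutoDetonate before calling Explode.
; Explode spawns particles and sound scaled by game volume and time dilation, applies radial damage with falloff, then destroys the actor.
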(event `self.ReceiveBeginPlay`
  (bind _asbp_player_pawn (cast `/Game/VRLocomotionTemplate/Core/Characters/BP_PlayerPawn` (`GameplayStatics.GetPlayerPawn` 0)))
  (set `self.Player` _asbp_player_pawn)
  (bind _asbp_vrgamemode (cast `/Game/VRLocomotionTemplate/Core/GameModes/BP_VRGamemode` (`GameplayStatics.GetGameMode`)))
  (set `self.Gamemode` _asbp_vrgamemode)
  (`KismetSystemLibrary.Delay` 0.1)
  (`KismetSystemLibrary.Delay` (`self.fAutoDetonate`))
  (`self.Explode`))

(event `self.ReceiveTick`
  (params (DeltaSeconds :type "Float (single-precision)")))

(fn `Explode`
  (bind (_returnvalue_location _returnvalue_rotation) (`KismetMathLibrary.BreakTransform` (`self.GetTransform`)))
  (bind _damage (`self.Damage`))
  (`GameplayStatics.SpawnEmitterAtLocation` "/Game/VRLocomotionTemplate/ParticleSystems/Explosion/Particles/P_Explosion.P_Explosion" _returnvalue_location _returnvalue_rotation (1.5 1.5 1.5))
  (`GameplayStatics.SpawnSoundAtLocation` "/Game/VRLocomotionTemplate/Audio/SoundFiles/Weapon/7B_Grenade_Explosion_M_V1_RO.7B_Grenade_Explosion_M_V1_RO" _returnvalue_location (struct) (`/Game/VRLocomotionTemplate/Core/GameModes/BP_VRGamemode.GameVolume` (`self.Gamemode`)) (`GameplayStatics.GetGlobalTimeDilation`) 0.0 null null)
  (`GameplayStatics.ApplyRadialDamageWithFalloff` :`BaseDamage` _damage :`MinimumDamage` (/ _damage 5.0) :`Origin` (`self.K2_GetActorLocation`) :`DamageInnerRadius` 100.0 :`DamageOuterRadius` 300.0 :`DamageTypeClass` "/Script/Engine.DamageType" :`DamageCauser` null :`InstigatedByController` null)
  (`self.K2_DestroyActor`))

(fn `UserConstructionScript`)