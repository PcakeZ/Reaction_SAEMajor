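; VR game mode that drives sample-based recording and replay scrubbing, with time frozen outside of both.
; BeginPlay caches the player pawn and converts the recording settings into a sample count and interval.
; While recording, a Delay-throttled Tick calls the record and play dispatchers.
; Otherwise, holding one scrub direction restores normal time and steps a clamped sample index for readback, while neither or both sets time dilation to zero.
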(event `self.ReceiveBeginPlay`
  (bind _asbp_player_pawn (cast `/Game/VRLocomotionTemplate/Core/Characters/BP_PlayerPawn` (`GameplayStatics.GetPlayerPawn` 0)))
  (set `self.Player` _asbp_player_pawn)
  (set `self.RecordTime` (* (`self.SamplesPerSecond`) (`self.RecordTime`)))
  (set `self.SamplesPerSecond` (/ 1.0 (`self.SamplesPerSecond`))))

(event `self.ReceiveTick`
  (params (DeltaSeconds :type "Float (single-precision)"))
  (bind _currentsample (`self.CurrentSample`))
  (bind _leftscrubing (`self.LeftScrubing`))
  (bind _rightscrubing (`self.RightScrubing`))
  (if (`self.bRecording`)
    ;[1 0 0] Call Actors Record
    (`KismetSystemLibrary.Delay` (`self.SamplesPerSecond`))
    (`self.RecordSample`)
    (`self.PlaySample`)
    (else
      ;[0 1 0.9916] Record Scrubing
      (if (and (or _leftscrubing _rightscrubing) (not (and _leftscrubing _rightscrubing)))
        (`GameplayStatics.SetGlobalTimeDilation` 1.0)
        (`KismetSystemLibrary.Delay` (`self.SamplesPerSecond`))
        (if (`self.LeftScrubing`)
          (set `self.CurrentSample` (`KismetMathLibrary.Clamp` (- (`self.CurrentSample`) 1) 0 (`self.ReplayLength`)))
          (else
            (set `self.CurrentSample` (`KismetMathLibrary.Clamp` (+ (`self.CurrentSample`) 1) 0 (`self.ReplayLength`)))))
        (`self.ReadSample` _currentsample)
        (`KismetSystemLibrary.PrintString` (`KismetStringLibrary.Conv_IntToString` _currentsample))
        (else
          (`GameplayStatics.SetGlobalTimeDilation` 0.0))))))

(fn `UserConstructionScript`)