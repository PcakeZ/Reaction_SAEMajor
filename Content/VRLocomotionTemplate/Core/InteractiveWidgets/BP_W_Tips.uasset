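; BP_W_Tips is an actor in the VR locomotion template that shows a tip widget facing the player.
; On BeginPlay it passes its CurrentTip to the UI_Tips user widget and caches the BP_PlayerPawn.
; Every Tick it rotates the widget component toward the pawn's camera with a look-at rotation, so the tip follows the viewer like a billboard.
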(event `self.ReceiveBeginPlay`
  (bind _asui_tips (cast `/Game/VRLocomotionTemplate/Widgets/Tips/UI_Tips` (`WidgetComponent.GetUserWidgetObject` (`self.Widget`))))
  (set `self.WidgetRef` _asui_tips)
  (set `/Game/VRLocomotionTemplate/Widgets/Tips/UI_Tips.CurrentTip` (`self.CurrentTip`) (`self.WidgetRef`))
  (bind _asbp_player_pawn (cast `/Game/VRLocomotionTemplate/Core/Characters/BP_PlayerPawn` (`GameplayStatics.GetPlayerPawn` 0)))
  (set `self.Player` _asbp_player_pawn))

(event `self.ReceiveTick`
  (params (DeltaSeconds :type "Float (single-precision)"))
  (`SceneComponent.K2_SetWorldRotation` (`self.Widget`) (`KismetMathLibrary.FindLookAtRotation` (`SceneComponent.K2_GetComponentLocation` (`self.Widget`)) (`SceneComponent.K2_GetComponentLocation` (`/Game/VRLocomotionTemplate/Core/Characters/BP_PlayerPawn.Camera` (`self.Player`)))) false false))

(fn `UserConstructionScript`)