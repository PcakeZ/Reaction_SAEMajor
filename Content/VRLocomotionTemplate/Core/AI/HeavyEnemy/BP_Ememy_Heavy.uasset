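; Heavy enemy AI for a VR game that carries a spawned minigun in its right hand, fires bursts at the player and dies from any damage.
; Delay-throttled Tick checks range and traces to the player's head, moving toward the player if blocked or stopping to shoot once the cooldown expires.
; While shooting it yaws toward the player and launches impulse-driven bullets at the head with random spread until the burst empties.
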(event `self.ReceiveBeginPlay`
  (bind _asbp_player_pawn (cast `/Game/VRLocomotionTemplate/Core/Characters/BP_PlayerPawn` (`GameplayStatics.GetPlayerPawn` 0)))
  (set `self.Player` _asbp_player_pawn)
  (set `self.MaxWalkSpeedRef` (`CharacterMovementComponent.MaxWalkSpeed` (`self.CharacterMovement`)))
  (bind _returnvalue (`|SpawnActorFromClass` "/Game/VRLocomotionTemplate/Core/Weapons/BP_Minigun.BP_Minigun_C" (`SceneComponent.GetRelativeTransform` (`self.MinigunPos`)) "Undefined" "OverrideRootScale" null null))
  (bind _output_get (set `self.MiniGun` _returnvalue))
  (`self.K2_AttachToComponent` _returnvalue (`self.Mesh`) "RightHandSocket" "KeepRelative" "KeepRelative" "KeepRelative" true)
  (`self.K2_AttachToComponent` _output_get (`self.Mesh`) "RightHandSocket" "KeepRelative" "KeepRelative" "KeepRelative" true))

(event `self.ReceiveTick`
  (params (DeltaSeconds :type "Float (single-precision)"))
  (bind _returnvalue (`self.K2_GetActorLocation`))
  (bind _mesh (`self.Mesh`))
  (bind _player (`self.Player`))
  (bind _mesh_2 (`self.Mesh`))
  (bind _mesh_3 (`self.Mesh`))
  (bind (_returnvalue_roll _returnvalue_pitch _returnvalue_yaw) (`KismetMathLibrary.BreakRotator` (`KismetMathLibrary.FindLookAtRotation` (`self.K2_GetActorLocation`) (`self.K2_GetActorLocation` (`self.Player`)))))
  (set `self.CurrentShootCooldown` (- (`self.CurrentShootCooldown`) DeltaSeconds))
  (if (`self.IsShooting`)
    (`SkeletalMeshComponent.SetPlayRate` _mesh 0.5)
    (`self.K2_SetActorRotation` (`KismetMathLibrary.MakeRotator` 0.0 0.0 _returnvalue_yaw))
    (`KismetSystemLibrary.Delay` 0.1)
    (if (> (`self.CurrentBulletNum`) 0)
      (`self.Shoot`)
      (else
        (set `CharacterMovementComponent.MaxWalkSpeed` (`self.MaxWalkSpeedRef`) (`self.CharacterMovement`))
        (set `self.CurrentShootCooldown` (`self.ShootCooldown`))
        (set `self.IsShooting` false)
        (`SkeletalMeshComponent.SetAnimation` _mesh_3 "/Game/VRLocomotionTemplate/Models/TempHeavy/Rifle_Crouch_Walk_Anim.Rifle_Crouch_Walk_Anim")
        (`SkeletalMeshComponent.Play` _mesh_3 true)))
    (else
      (`SkeletalMeshComponent.SetPlayRate` _mesh (/ (`KismetMathLibrary.VSize` (`self.GetVelocity`)) 70.0))
      (`KismetSystemLibrary.Delay` 1.0)
      (if (<= (`KismetMathLibrary.Vector_Distance` (`self.K2_GetActorLocation` _player) _returnvalue) (`self.MinDistance`))
        (bind (_outhit _returnvalue_2) (`KismetSystemLibrary.LineTraceSingleForObjects` :`Start` _returnvalue :`End` (`SceneComponent.K2_GetComponentLocation` (`/Game/VRLocomotionTemplate/Core/Characters/BP_PlayerPawn.HeadHitBox` _player)) :`ObjectTypes` (`self.TraceObjectTypes`) :`DrawDebugType` "ForDuration" :`DrawTime` 1.0))
        (if _returnvalue_2
          (if (== (`.HitActor` (`GameplayStatics.BreakHitResult` _outhit)) (`self.Player`))
            (`MovementComponent.StopMovementImmediately` (`self.CharacterMovement`))
            (if (< (`self.CurrentShootCooldown`) 0.0)
              (set `self.IsShooting` true)
              (set `self.CurrentBulletNum` (`self.BulletNum`))
              (set `CharacterMovementComponent.MaxWalkSpeed` 0.0 (`self.CharacterMovement`))
              (`SkeletalMeshComponent.SetAnimation` _mesh_2 "/Game/VRLocomotionTemplate/Models/TempHeavy/Gunplay.Gunplay")
              (`SkeletalMeshComponent.Play` _mesh_2 true))
            (else
              (`|AIMoveTo` self (0.0 0.0 0.0) (`self.Player`)))))))))

(event `self.ReceiveAnyDamage`
  (params (Damage :type "Float (single-precision)") (DamageType :type "DamageType Object Reference") (InstigatedBy :type "Controller Object Reference") (DamageCauser :type "Actor Object Reference"))
  (`self.K2_DestroyActor`))

(fn `Shoot`
  (bind (_inaccuracy_roll _inaccuracy_pitch _inaccuracy_yaw) (`KismetMathLibrary.BreakRotator` (`self.inaccuracy`)))
  (bind (_returnvalue_location _returnvalue_rotation) (`KismetMathLibrary.BreakTransform` (`SceneComponent.K2_GetComponentToWorld` (`/Game/VRLocomotionTemplate/Core/Weapons/BP_Minigun.ShootingPos` (`self.MiniGun`)))))
  (bind (_returnvalue_roll _returnvalue_pitch _returnvalue_yaw) (`KismetMathLibrary.BreakRotator` (`KismetMathLibrary.FindLookAtRotation` (`SceneComponent.K2_GetComponentLocation` (`self.ShootingPos`)) (`SceneComponent.K2_GetComponentLocation` (`/Game/VRLocomotionTemplate/Core/Characters/BP_PlayerPawn.HeadHitBox` (`self.Player`))))))
  (bind _returnvalue (`|SpawnActorFromClass` "/Game/VRLocomotionTemplate/Core/Weapons/BP_Bullet_Enemy.BP_Bullet_Enemy_C" (`KismetMathLibrary.MakeTransform` _returnvalue_location _returnvalue_rotation (0.03 0.015 0.015)) "Undefined" "OverrideRootScale" null null))
  (`PrimitiveComponent.AddImpulse` (`/Game/VRLocomotionTemplate/Core/Weapons/BP_Bullet_Enemy.Cube` _returnvalue) (* (`KismetMathLibrary.GetForwardVector` (`KismetMathLibrary.MakeRotator` _returnvalue_roll (+ _returnvalue_pitch (`KismetMathLibrary.RandomFloatInRange` (* _inaccuracy_pitch -1.0) _inaccuracy_pitch)) (+ _returnvalue_yaw (`KismetMathLibrary.RandomFloatInRange` (* _inaccuracy_yaw -1.0) _inaccuracy_yaw)))) (`self.BulletSpeed`)) "None" true)
  (`GameplayStatics.PlaySoundAtLocation` "/Game/VRLocomotionTemplate/Audio/SoundFiles/Weapon/29_Minigun_Fire_M_V1_RO.29_Minigun_Fire_M_V1_RO" (`SceneComponent.K2_GetComponentLocation` (`self.ShootingPos`)) (struct) 1.0 1.0 0.0 null null null)
  (`/Engine/EditorBlueprintResources/StandardMacros.DecrementInt` (`self.CurrentBulletNum`)))

(fn `UserConstructionScript`)