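; Enemy drone character for a VR game that caches the player pawn on BeginPlay and is destroyed by any damage.
; Shoot fires a bullet at the player's head hitbox using an impulse with random pitch and yaw spread, plus a bang sound.
; Hovering by downward trace, AI chase and line-of-sight burst firing with cooldown are drafted but disconnected.
; Tick is empty and Shoot's only call is in that dead logic, so the drone neither moves nor fires itself.
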(event `self.ReceiveBeginPlay`
  (bind _asbp_player_pawn (cast `/Game/VRLocomotionTemplate/Core/Characters/BP_PlayerPawn` (`GameplayStatics.GetPlayerPawn` 0)))
  (set `self.Player` _asbp_player_pawn)
  (set `self.MaxWalkSpeedRef` (`CharacterMovementComponent.MaxWalkSpeed` (`self.CharacterMovement`))))

(event `self.ReceiveTick`
  (params (DeltaSeconds :type "Float (single-precision)")))

(event `self.ReceiveAnyDamage`
  (params (Damage :type "Float (single-precision)") (DamageType :type "DamageType Object Reference") (InstigatedBy :type "Controller Object Reference") (DamageCauser :type "Actor Object Reference"))
  (`self.K2_DestroyActor`))

(fn `Shoot`
  (bind (_inaccuracy_roll _inaccuracy_pitch _inaccuracy_yaw) (`KismetMathLibrary.BreakRotator` (`self.inaccuracy`)))
  (bind (_returnvalue_location _returnvalue_rotation) (`KismetMathLibrary.BreakTransform` (`SceneComponent.K2_GetComponentToWorld` (`self.ShootingPos`))))
  (bind (_returnvalue_roll _returnvalue_pitch _returnvalue_yaw) (`KismetMathLibrary.BreakRotator` (`KismetMathLibrary.FindLookAtRotation` (`SceneComponent.K2_GetComponentLocation` (`self.ShootingPos`)) (`SceneComponent.K2_GetComponentLocation` (`/Game/VRLocomotionTemplate/Core/Characters/BP_PlayerPawn.HeadHitBox` (`self.Player`))))))
  (bind _returnvalue (`|SpawnActorFromClass` "/Game/VRLocomotionTemplate/Core/Weapons/BP_Bullet_Enemy.BP_Bullet_Enemy_C" (`KismetMathLibrary.MakeTransform` _returnvalue_location _returnvalue_rotation (0.03 0.015 0.015)) "Undefined" "OverrideRootScale" null null))
  (`PrimitiveComponent.AddImpulse` (`/Game/VRLocomotionTemplate/Core/Weapons/BP_Bullet_Enemy.Cube` _returnvalue) (* (`KismetMathLibrary.GetForwardVector` (`KismetMathLibrary.MakeRotator` _returnvalue_roll (+ _returnvalue_pitch (`KismetMathLibrary.RandomFloatInRange` (* _inaccuracy_pitch -1.0) _inaccuracy_pitch)) (+ _returnvalue_yaw (`KismetMathLibrary.RandomFloatInRange` (* _inaccuracy_yaw -1.0) _inaccuracy_yaw)))) (`self.BulletSpeed`)) "None" true)
  (`GameplayStatics.PlaySoundAtLocation` "/Game/VRLocomotionTemplate/Audio/S_Bang.S_Bang" (`SceneComponent.K2_GetComponentLocation` (`self.ShootingPos`)) (struct) 1.0 1.0 0.0 null null null)
  (`/Engine/EditorBlueprintResources/StandardMacros.DecrementInt` (`self.CurrentBulletNum`)))

(fn `UserConstructionScript`)