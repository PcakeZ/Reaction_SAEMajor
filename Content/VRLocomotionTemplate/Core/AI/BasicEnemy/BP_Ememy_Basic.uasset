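; Basic VR-template enemy that spawns a pistol in its right hand, hunts the player pawn and is destroyed by any damage.
; A Delay on Tick throttles its logic, which line-traces to the player's head hitbox within MinDistance until it latches SeePlayer.
; It then plays a run animation scaled by speed, chases via AIMoveTo and fires the pistol on a delay.
; Direct bullet-spawning code in Shoot is unreachable.
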(event `self.ReceiveBeginPlay`
  (bind _pistolpos (`self.PistolPos`))
  (bind _asbp_player_pawn (cast `/Game/VRLocomotionTemplate/Core/Characters/BP_PlayerPawn` (`GameplayStatics.GetPlayerPawn` 0)))
  (set `self.Player` _asbp_player_pawn)
  (bind _returnvalue (`|SpawnActorFromClass` "/Game/VRLocomotionTemplate/Core/Weapons/BP_Pistol.BP_Pistol_C" (`KismetMathLibrary.MakeTransform` (0.0 -6.0 5.0) (`KismetMathLibrary.MakeRotator` 90.0 0.0 -90.0) (.scale (`SceneComponent.GetRelativeTransform` (`self.PistolPos`)))) "Undefined" "OverrideRootScale" null null))
  (bind _output_get (set `self.Weapon` _returnvalue))
  (message `/Game/VRLocomotionTemplate/Core/Interactables/I_Interactable.StartInteract` _output_get _pistolpos _pistolpos)
  (`SceneComponent.K2_AttachToComponent` _pistolpos (`self.Mesh`) "RightHandSocket" "KeepRelative" "KeepRelative" "KeepRelative" true))

(event `self.ReceiveTick`
  (params (DeltaSeconds :type "Float (single-precision)"))
  (bind _returnvalue (`self.K2_GetActorLocation`))
  (bind _mesh (`self.Mesh`))
  (bind _player (`self.Player`))
  (`KismetSystemLibrary.Delay` 1.0)
  (if (`self.SeePlayer`)
    (`SkeletalMeshComponent.SetPlayRate` (`self.Mesh`) (/ (`KismetMathLibrary.VSize` (`self.GetVelocity`)) 300.0))
    (`|AIMoveTo` self (0.0 0.0 0.0) (`self.Player`)
      (:`then`
        (`KismetSystemLibrary.Delay` 3.0)
        (`self.Shoot`)))
    (elif (<= (`KismetMathLibrary.Vector_Distance` (`self.K2_GetActorLocation` _player) _returnvalue) (`self.MinDistance`))
      (bind (_outhit _returnvalue_2) (`KismetSystemLibrary.LineTraceSingleForObjects` :`Start` _returnvalue :`End` (`SceneComponent.K2_GetComponentLocation` (`/Game/VRLocomotionTemplate/Core/Characters/BP_PlayerPawn.HeadHitBox` _player)) :`ObjectTypes` (`self.TraceObjectTypes`) :`DrawTime` 1.0))
      (if _returnvalue_2
        (if (== (`.HitActor` (`GameplayStatics.BreakHitResult` _outhit)) (`self.Player`))
          (set `self.SeePlayer` true)
          (`SkeletalMeshComponent.SetAnimation` _mesh "/Game/VRLocomotionTemplate/Models/EnemyBasic/Pistol_Run__3_.Pistol_Run__3_")
          (`SkeletalMeshComponent.Play` _mesh true))))))

(event `self.ReceiveAnyDamage`
  (params (Damage :type "Float (single-precision)") (DamageType :type "DamageType Object Reference") (InstigatedBy :type "Controller Object Reference") (DamageCauser :type "Actor Object Reference"))
  (`self.K2_DestroyActor`))

(fn `Shoot`
  (`/Game/VRLocomotionTemplate/Core/Weapons/BP_Pistol.Shoot` (`self.Weapon`)))

(fn `UserConstructionScript`)